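; BP_Campfire is a campfire actor with optional smoke, mesh and light, plus an interaction prompt.
; The construction script hides each part whose include flag is off, with the light hidden through LightRotator and its children.
; Focus shows InteractInfo until a retriggerable delay expires or UnFocus hides it, while PickUp always returns false.
; A sine-driven rotation for light movement is present but unconnected, so it never runs.
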(event `self.ReceiveTick`
  (params (DeltaSeconds :type "Float (single-precision)")))

(event `/Game/CombatSystem/BluePrints/UserInterface/BPI_Interact.Focus`
  (bind _interactinfo (`self.InteractInfo`))
  (`SceneComponent.SetVisibility` _interactinfo true false)
  (`KismetSystemLibrary.RetriggerableDelay` 0.5)
  (`SceneComponent.SetVisibility` _interactinfo false false))

(event `/Game/CombatSystem/BluePrints/UserInterface/BPI_Interact.UnFocus`
  (`SceneComponent.SetVisibility` (`self.InteractInfo`) false false))

(fn `PickUp`
  (returns (Dummy :type Boolean))
  (return false))

(fn `UserConstructionScript`
  (if (not (`self.IncludeSmoke`))
    (`SceneComponent.SetVisibility` (`self.P_Smoke`) false false))
  (if (not (`self.IncludeMesh`))
    (`SceneComponent.SetVisibility` (`self.Campfire`) false false))
  (if (not (`self.IncludeLight`))
    (`SceneComponent.SetVisibility` (`self.LightRotator`) false true)))