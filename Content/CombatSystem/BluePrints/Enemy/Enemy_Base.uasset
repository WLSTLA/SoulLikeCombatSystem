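; Base enemy AI character for melee combat against the player, handling hits, blocks, stuns, executions and death.
; On BeginPlay it caches its AI controller, sets up the health widget and attaches a spawned weapon that drives montage selection and hit collision.
; Combat state passes to the AI through blackboard enums, while components supply montages and health.
; Death stops the behavior tree and dissolves mesh and weapon, with a separate ragdoll path.
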(event `self.ReceiveBeginPlay`
  (bind _bpc_dissolveeffectcomponent (`self.BPC_DissolveEffectComponent`))
  (bind _bpc_collisionhandle (`self.BPC_CollisionHandle`))
  (bind ((`WeaponType_29_34EA040D45CE8853B8FEC6A08C8B7672` _weapontype) (`EquipSocket_16_BDEC2EBE43ABEEA9BD9EB79A98D26426` _equipsocket)) (break `/Game/CombatSystem/BluePrints/Structures/S_WeaponInfo` (`/Game/CombatSystem/BluePrints/Core/Item/Weapon/BP_WeaponMaster.WeaponInfo` (`self.WeaponRef`))))
  ;[1 1 1] BeginPlay
  (`|ExecutionSequence`
    (:`then_0`
      (bind _asaic_enemy_controller (cast `/Game/CombatSystem/BluePrints/Enemy/AIC_EnemyController` (`AIBlueprintHelperLibrary.GetAIController` self)))
      (set `self.AIController` _asaic_enemy_controller))
    (:`then_1`
      (bind _returnvalue (`|CreateWidget` "/Game/CombatSystem/HUD/Widgets/UMG_EnemyBase.UMG_EnemyBase_C"))
      (`WidgetComponent.SetWidget` (`self.HealthWidget`) _returnvalue)
      (`/Game/CombatSystem/BluePrints/Components/BPC_StatsManager.InitialStats` (`self.BPC_Health`) (`/Game/CombatSystem/HUD/Widgets/UMG_EnemyBase.Health1` _returnvalue) (`/Game/CombatSystem/HUD/Widgets/UMG_EnemyBase.Health2` _returnvalue)))
    (:`then_2`
      (bind _returnvalue_2 (`|SpawnActorFromClass` (`self.WeaponClass`) (`KismetMathLibrary.MakeTransform` (0.0 0.0 0.0)) "Undefined" "OverrideRootScale" null null))
      (bind _asbp_weapon_master (cast `/Game/CombatSystem/BluePrints/Core/Item/Weapon/BP_WeaponMaster` _returnvalue_2))
      (bind _output_get (set `self.WeaponRef` _asbp_weapon_master))
      (`self.K2_AttachToComponent` _output_get (`self.Mesh`) _equipsocket "SnapToTarget" "SnapToTarget" "SnapToTarget" true)
      (`/Game/CombatSystem/BluePrints/Components/BPC_MontagesManager.UpdateWeaponType` (`self.BPC_MontagesManager`) _weapontype)
      (`/Game/CombatSystem/BluePrints/Components/BPC_CollisionHandle.UpdateWeaponAndSocet` _bpc_collisionhandle (`/Game/CombatSystem/BluePrints/Core/Item/BP_ItemMaster.ItemMesh` (`self.WeaponRef`)))
      (add `/Game/CombatSystem/BluePrints/Components/BPC_CollisionHandle.OnHit` _bpc_collisionhandle (`|CreateDelegate` :!event `OnHit`))
      (`/Game/CombatSystem/BluePrints/Components/BPC_DissolveEffectComponent.GetOnwerNeedDissolveMesh` _bpc_dissolveeffectcomponent (`self.Mesh`))
      (`/Game/CombatSystem/BluePrints/Components/BPC_DissolveEffectComponent.GetOnwerNeedDissolveMesh` _bpc_dissolveeffectcomponent (`/Game/CombatSystem/BluePrints/Core/Item/BP_ItemMaster.ItemMesh` (`self.WeaponRef`))))
    (:`then_3`
      (bind _asplayer (cast `/Game/CombatSystem/BluePrints/Player/Player` (`GameplayStatics.GetPlayerCharacter` 0)))
      (add `/Game/CombatSystem/BluePrints/Player/Player.PlayerDeathDispatcher` _asplayer (delegate `ResetBehavior`)))
    (:`then_4`
      (bind _asabp_enemy_base (cast `/Game/CombatSystem/BluePrints/Enemy/ABP_EnemyBase` (`SkeletalMeshComponent.GetAnimInstance` (`self.Mesh`))))
      (set `self.EnemyAnimRef` _asabp_enemy_base))))

(event `ResetBehavior`
  ;[1 1 1] BeginPlay
  (`/Game/CombatSystem/BluePrints/Enemy/AIC_EnemyController.ResetPerception` (`self.AIController`)))

(fn `Block`
  (params (AttackType :type "/Game/CombatSystem/BluePrints/Enumerations/Character/E_AttackType Enum" :default "NewEnumerator4") (HitLocation :type "Vector Structure"))
  (bind (_blockmontage _success_) (`self.GetBlockMontage` AttackType))
  (if _success_
    (`self.PlayAnimMontage` _blockmontage)
    (`self.SpawnEmitter` "/Game/CombatSystem/FPX/P_Imp_Metal.P_Imp_Metal" HitLocation (struct :`Pitch` 10.0) (1.0 1.0 1.0))
    (return)
    (else
      ;[1 1 1] 确保播放动画
      (`self.PlayAnimMontage` "/Game/CombatSystem/BluePrints/Player/GreatSwordAinm/Montages/Block/GreatSword_Defense_Hit_Montage.GreatSword_Defense_Hit_Montage")
      (return))))

(fn `CanBeDestroyEvent`
  (returns (Dumy :type Boolean))
  (`self.K2_DestroyActor`)
  (return false))

(fn `Death`
  (params (`PlayDeadMontage?` :type Boolean))
  (bind _aicontroller (`self.AIController`))
  (set `self.Dead` true)
  (if `PlayDeadMontage?`
    (bind (_deadmontage _success_) (`self.GetDeadMontage`))
    (if _success_
      (`self.PlayAnimMontage` _deadmontage)
      ;[1 1 1] 设置黑板中的Enum为Dead
      (`/Game/CombatSystem/BluePrints/Enemy/AIC_EnemyController.SetEnumInBlackboard` _aicontroller (`/Game/CombatSystem/BluePrints/Enemy/AIC_EnemyController.GetAIStateKey` _aicontroller) (enumliteral `/Game/CombatSystem/BluePrints/Enumerations/AI/E_AIState` "NewEnumerator4") :!label _label)
      ;[1 1 1] Set Movement
      (`CharacterMovementComponent.DisableMovement` (`self.CharacterMovement`))
      ;[1 1 1] StopBehaviorTree
      (`BrainComponent.StopLogic` (`AIController.BrainComponent` (`self.AIController`)) "")
      ;[1 1 1] 脱离控制
      (`Controller.UnPossess` (`self.AIController`))
      ;[1 1 1] SetWidgets And Dispatcher
      (`self.SetAllWidgets` false)
      (`self.AIDeathDispatcher`)
      ;[1 1 1] Dissolve Effect
      (`/Game/CombatSystem/BluePrints/Components/BPC_DissolveEffectComponent.BeginDissolved` (`self.BPC_DissolveEffectComponent`))
      (return))
    (else
      (goto _label))))

(fn `ExecutionHandle`
  (params (ExecutedIndex :type Integer) (ExecutorWeaponType :type "/Game/CombatSystem/BluePrints/Enumerations/Character/E_WeaponType Enum" :default "NewEnumerator3"))
  (returns (Dummy :type Boolean))
  (bind _aicontroller (`self.AIController`))
  ;[1 1 1] MontagePlay
  (bind (_executmontage _success_) (`self.GetExecutionMontage` ExecutedIndex ExecutorWeaponType))
  (if _success_
    (`self.PlayAnimMontage` _executmontage)
    ;[1 1 1] 设置黑板中的Enum为Dead
    (`/Game/CombatSystem/BluePrints/Enemy/AIC_EnemyController.SetEnumInBlackboard` _aicontroller (`/Game/CombatSystem/BluePrints/Enemy/AIC_EnemyController.GetAIStateKey` _aicontroller) (enumliteral `/Game/CombatSystem/BluePrints/Enumerations/AI/E_AIState` "NewEnumerator4"))
    ;[1 1 1] SetCollision
    (`CharacterMovementComponent.DisableMovement` (`self.CharacterMovement`))
    (`PrimitiveComponent.SetCollisionResponseToChannel` (`self.CapsuleComponent`) "ECC_Pawn" "ECR_Overlap")
    ;[1 1 1] Update HealthWidge
    (`/Game/CombatSystem/BluePrints/Components/BPC_StatsManager.Update Stat` (`self.BPC_Health`) -100.0 false)
    (return false)
    (else
      (`KismetSystemLibrary.PrintString` "Enemy获取处决动画失败"))))

(fn `GetAttackMontage`
  (params (AttackType :type "/Game/CombatSystem/BluePrints/Enumerations/Character/E_AttackType Enum" :default "NewEnumerator4") (AttackIndex :type Integer) (`SpecifyAttackMontage?` :type Boolean))
  (returns (AttackMontage :type "AnimMontage Object Reference") (`Success?` :type Boolean))
  (locals (LocalLastIndex :type Integer :default 0) (LocalAttackAction :type "/Game/CombatSystem/BluePrints/Enumerations/Character/E_MontageAction Enum" :default "NewEnumerator0"))
  (bind _aicontroller (`self.AIController`))
  (`/Game/CombatSystem/BluePrints/Enemy/AIC_EnemyController.SetEnumInBlackboard` _aicontroller (`/Game/CombatSystem/BluePrints/Enemy/AIC_EnemyController.GetAttackTypeKey` _aicontroller) AttackType)
  (bind _output_get (set `local.LocalAttackAction` (`/Game/CombatSystem/BluePrints/FunctionLibrary/BPF_CombatBaseLibrary.ChangeAttackTypeToAction` AttackType)))
  (bind (_isfind_ _last_index) (`/Game/CombatSystem/BluePrints/Components/BPC_MontagesManager.GetActionLastIndex` (`self.BPC_MontagesManager`) _output_get "NewEnumerator3"))
  (if _isfind_
    (if (`local.SpecifyAttackMontage?`)
      ;[1 1 1] 指定一个特定攻击
      (bind (_action _success_) (`/Game/CombatSystem/BluePrints/Components/BPC_MontagesManager.GetMontageForAction` (`self.BPC_MontagesManager`) (`local.LocalAttackAction`) (`KismetMathLibrary.Clamp` (`local.AttackIndex`) 0 _last_index) "NewEnumerator3"))
      (return _action _success_)
      (else
        (bind (_action_2 _success__2) (`/Game/CombatSystem/BluePrints/Components/BPC_MontagesManager.GetMontageForAction` (`self.BPC_MontagesManager`) (`local.LocalAttackAction`) (`KismetMathLibrary.RandomIntegerInRange` 0 _last_index) "NewEnumerator3"))
        (return _action_2 _success__2)))
    (else
      (return null false))))

(fn `GetBlockMontage`
  (params (AttackType :type "/Game/CombatSystem/BluePrints/Enumerations/Character/E_AttackType Enum" :default "NewEnumerator4"))
  (returns (BlockMontage :type "AnimMontage Object Reference") (`Success?` :type Boolean))
  (locals (LocalAttackType :type "/Game/CombatSystem/BluePrints/Enumerations/Character/E_AttackType Enum" :default "NewEnumerator4") (LocalLastIndex :type Integer))
  (bind _output_get (set `local.LocalAttackType` AttackType))
  (switch `/Game/CombatSystem/BluePrints/Enumerations/Character/E_AttackType` _output_get
    (:`NewEnumerator0`
      (bind (_isfind_ _last_index) (`/Game/CombatSystem/BluePrints/Components/BPC_MontagesManager.GetActionLastIndex` (`self.BPC_MontagesManager`) "NewEnumerator5" "NewEnumerator3"))
      (if _isfind_
        (bind _output_get_2 (set `local.LocalLastIndex` _last_index))
        (bind (_action _success_) (`/Game/CombatSystem/BluePrints/Components/BPC_MontagesManager.GetMontageForAction` (`self.BPC_MontagesManager`) "NewEnumerator5" (`KismetMathLibrary.RandomIntegerInRange` 0 (- _output_get_2 1)) "NewEnumerator3"))
        (return _action _success_)))
    (:`NewEnumerator1`
      ;[1 1 1] DefenseBorken
      (bind (_isfind__2 _last_index_2) (`/Game/CombatSystem/BluePrints/Components/BPC_MontagesManager.GetActionLastIndex` (`self.BPC_MontagesManager`) "NewEnumerator5" "NewEnumerator3" :!label _label))
      (if _isfind__2
        (bind _output_get_3 (set `local.LocalLastIndex` _last_index_2))
        (bind (_action_2 _success__2) (`/Game/CombatSystem/BluePrints/Components/BPC_MontagesManager.GetMontageForAction` (`self.BPC_MontagesManager`) "NewEnumerator5" _output_get_3 "NewEnumerator3"))
        (return _action_2 _success__2)))
    (:`NewEnumerator3`
      (goto _label))
    (:`NewEnumerator2`
      (goto _label))))

(fn `GetDamage`
  (returns (Damage :type "Float (double-precision)"))
  (bind (_lightattackdamagemultipies _heavyattackdamagemultipies _thrustattackdamagemultipies _specialattackdamagemultipies) (break `/Game/CombatSystem/BluePrints/Structures/S_DamageStat` (`self.GetStatInfo`)))
  (return (* (`.BaseDamage_9_6FC6DC044EA9E86C118075B9D788D381` (break `/Game/CombatSystem/BluePrints/Structures/S_WeaponInfo` (`/Game/CombatSystem/BluePrints/Core/Item/Weapon/BP_WeaponMaster.WeaponInfo` (`self.WeaponRef`)))) (select `/Game/CombatSystem/BluePrints/Enumerations/Character/E_AttackType` (`self.GetAttackType`) :`NewEnumerator0` _lightattackdamagemultipies :`NewEnumerator1` _heavyattackdamagemultipies :`NewEnumerator3` _thrustattackdamagemultipies :`NewEnumerator2` _specialattackdamagemultipies))))

(fn `GetDeadMontage`
  (returns (DeadMontage :type "AnimMontage Object Reference") (`Success?` :type Boolean))
  (bind (_isfind_ _last_index) (`/Game/CombatSystem/BluePrints/Components/BPC_MontagesManager.GetActionLastIndex` (`self.BPC_MontagesManager`) "NewEnumerator16" "NewEnumerator3"))
  (if _isfind_
    (bind (_action _success_) (`/Game/CombatSystem/BluePrints/Components/BPC_MontagesManager.GetMontageForAction` (`self.BPC_MontagesManager`) "NewEnumerator16" (`KismetMathLibrary.RandomIntegerInRange` 0 _last_index) "NewEnumerator3"))
    (return _action _success_)
    (else
      (return null false))))

(fn `GetExecutionMontage`
  (params (ExecutIndex :type Integer) (WeaponType :type "/Game/CombatSystem/BluePrints/Enumerations/Character/E_WeaponType Enum" :default "NewEnumerator3"))
  (returns (ExecutMontage :type "AnimMontage Object Reference") (`Success?` :type Boolean))
  (bind (_action _success_) (`/Game/CombatSystem/BluePrints/Components/BPC_MontagesManager.GetMontageForAction` (`self.BPC_MontagesManager`) "NewEnumerator14" ExecutIndex WeaponType))
  (if _success_
    (return _action _success_)
    (else
      (return null false))))

(fn `GetHitSound`
  (params (WeaponType :type "/Game/CombatSystem/BluePrints/Enumerations/Character/E_WeaponType Enum" :default "NewEnumerator3"))
  (returns (AudioType :type "SoundBase Object Reference"))
  (return (select `/Game/CombatSystem/BluePrints/Enumerations/Character/E_WeaponType` WeaponType :`NewEnumerator4` "/Game/CombatSystem/Audio/Sword_Fighting/Sword/SoundCue/GreatSword_Hit_Flesh.GreatSword_Hit_Flesh" :`NewEnumerator7` "/Game/CombatSystem/Audio/Sword_Fighting/Sword/SoundCue/Sword_Hit_Flesh.Sword_Hit_Flesh" :`NewEnumerator8` "/Game/CombatSystem/Audio/Sword_Fighting/Sword/SoundCue/GreatSword_Hit_Flesh.GreatSword_Hit_Flesh" :!type "SoundBase Object Reference")))

(fn `GetImpactSound`
  (params (WeaponType :type "/Game/CombatSystem/BluePrints/Enumerations/Character/E_WeaponType Enum" :default "NewEnumerator3"))
  (returns (AudioType :type "SoundBase Object Reference"))
  (return (select `/Game/CombatSystem/BluePrints/Enumerations/Character/E_WeaponType` WeaponType :`NewEnumerator4` "/Game/CombatSystem/Audio/Weapons_woosh/SoundCue/GreatSword_Impact_Metalic_Light.GreatSword_Impact_Metalic_Light" :`NewEnumerator7` "/Game/CombatSystem/Audio/Weapons_woosh/SoundCue/TwinBlades_Impact_Metalic.TwinBlades_Impact_Metalic" :`NewEnumerator8` "/Game/CombatSystem/Audio/Weapons_woosh/SoundCue/GreatSword_Impact_Metalic_Light.GreatSword_Impact_Metalic_Light" :!type "SoundBase Object Reference")))

(fn `GetStatInfo`
  (returns (DamageStat :type "/Game/CombatSystem/BluePrints/Structures/S_DamageStat Structure"))
  (return (`.DamageStat_32_55BBA9BB440F08F91AD3CDB4E98C3554` (break `/Game/CombatSystem/BluePrints/Structures/S_Stat` (`self.AIStat`)))))

(fn `GetStunMontage`
  (params (HitDirection :type "/Game/CombatSystem/BluePrints/Enumerations/Character/E_HitDirection Enum" :default "NewEnumerator3") (AttackType :type "/Game/CombatSystem/BluePrints/Enumerations/Character/E_AttackType Enum" :default "NewEnumerator4"))
  (returns (StunMontage :type "AnimMontage Object Reference") (`GetSucees?` :type Boolean))
  (locals (LocalWeaponType :type "/Game/CombatSystem/BluePrints/Enumerations/Character/E_WeaponType Enum" :default "NewEnumerator3") (LocalHitDirection :type "/Game/CombatSystem/BluePrints/Enumerations/Character/E_HitDirection Enum" :default "NewEnumerator3") (LocalAttackType :type "/Game/CombatSystem/BluePrints/Enumerations/Character/E_AttackType Enum" :default "NewEnumerator4"))
  (bind _bpc_montagesmanager (`self.BPC_MontagesManager`))
  (set `local.LocalHitDirection` HitDirection)
  (switch `/Game/CombatSystem/BluePrints/Enumerations/Character/E_AttackType` AttackType
    (:`NewEnumerator0`
      ;[1 1 1] 轻击效果
      (bind (_action _success_) (`/Game/CombatSystem/BluePrints/Components/BPC_MontagesManager.GetMontageForAction` (`self.BPC_MontagesManager`) "NewEnumerator15" (select `/Game/CombatSystem/BluePrints/Enumerations/Character/E_HitDirection` (`local.LocalHitDirection`) :`NewEnumerator4` 1 :`NewEnumerator7` 2 :`NewEnumerator8` 3) "NewEnumerator3" :!label _label))
      (if _success_
        _
        (else
          (return null false))))
    (:`NewEnumerator1`
      ;[1 1 1] 重击效果
      (bind (_isfind_ _last_index) (`/Game/CombatSystem/BluePrints/Components/BPC_MontagesManager.GetActionLastIndex` _bpc_montagesmanager "NewEnumerator15" "NewEnumerator3" :!label _label_2))
      (bind (_action_2 _success__2) (`/Game/CombatSystem/BluePrints/Components/BPC_MontagesManager.GetMontageForAction` _bpc_montagesmanager "NewEnumerator15" _last_index "NewEnumerator3"))
      (if _success__2
        (return _action_2 true)
        (else
          (return null false))))
    (:`NewEnumerator3`
      (goto _label_2))
    (:`NewEnumerator2`
      (goto _label)))
  (return _action true))

(fn `GetWeaponInfo`
  (returns (WeaponInfo :type "/Game/CombatSystem/BluePrints/Structures/S_WeaponInfo Structure"))
  (bind _weaponref (`self.WeaponRef`))
  (if (`KismetSystemLibrary.IsValid` _weaponref)
    (return (`/Game/CombatSystem/BluePrints/Core/Item/Weapon/BP_WeaponMaster.WeaponInfo` _weaponref))))

(fn `HitHandle`
  (params (AttackCauser :type "Actor Object Reference") (Damage :type "Float (double-precision)") (HitDirection :type "/Game/CombatSystem/BluePrints/Enumerations/Character/E_HitDirection Enum" :default "NewEnumerator3") (WeaponType :type "/Game/CombatSystem/BluePrints/Enumerations/Character/E_WeaponType Enum" :default "NewEnumerator3") (DamageType :type "/Game/CombatSystem/BluePrints/Enumerations/Character/E_AttackType Enum" :default "NewEnumerator4") (HitLocation :type "Vector Structure") (HitBoneName :type Name))
  (returns (Dummy :type Boolean))
  (locals (LocalDamage :type "Float (double-precision)" :default 0.0) (LocalHitDirection :type "/Game/CombatSystem/BluePrints/Enumerations/Character/E_HitDirection Enum" :default "NewEnumerator3") (LocalAttackerWeaponType :type "/Game/CombatSystem/BluePrints/Enumerations/Character/E_WeaponType Enum" :default "NewEnumerator3") (LocalHitLocation :type "Vector Structure" :default (0.0 0.0 0.0)) (LocalAttackType :type "/Game/CombatSystem/BluePrints/Enumerations/Character/E_AttackType Enum" :default "NewEnumerator4") (LocalAttackCauser :type "/Game/CombatSystem/BluePrints/Player/Player Object Reference"))
  (bind (_asplayer _bsuccess) (cast `/Game/CombatSystem/BluePrints/Player/Player` AttackCauser :!pure true))
  (set `local.LocalHitLocation` HitLocation)
  (if (and (`KismetSystemLibrary.IsValid` AttackCauser) _bsuccess)
    (set `local.LocalAttackCauser` _asplayer)
    (set `local.LocalDamage` Damage)
    (set `local.LocalHitDirection` HitDirection)
    (set `local.LocalAttackerWeaponType` WeaponType)
    (set `local.LocalAttackType` DamageType)
    (if (`self.CanbeHit?`)
      (if (`self.CanBlock?` (`local.LocalHitDirection`))
        ;[1 1 1] Block
        (`self.Block` (`local.LocalAttackType`) (`local.LocalHitLocation`))
        ;[1 1 1] Impact
        (`/Game/CombatSystem/BluePrints/UserInterface/BPI_CanbeAttackable.Impact` (`local.LocalAttackCauser`))
        ;[1 1 1] CombatBehavior
        (`self.SetCombatBehavior` "NewEnumerator2")
        (else
          ;[1 1 1] 被攻击了就设置Player
          (`self.SetTargetOnPerception` (`local.LocalAttackCauser`))
          (`self.Stun` (`local.LocalHitDirection`) (`local.LocalHitLocation`) (`local.LocalAttackType`) (`local.LocalAttackerWeaponType`))
          ;[1 1 1] PlayHitSound
          (`self.PlaySound` (`self.GetHitSound` (`local.LocalAttackerWeaponType`)) (`local.LocalHitLocation`))
          ;[1 1 1] CombatBehavior
          (`self.SetCombatBehavior` "NewEnumerator2")
          (bind _isvalueempty_ (`/Game/CombatSystem/BluePrints/Components/BPC_StatsManager.Update Stat` (`self.BPC_Health`) (* (`local.LocalDamage`) -1.0) false))))
      (if _isvalueempty_
        (`self.Death` true)
        (return false)
        (else
          (return false))))))

(fn `Impact`
  (returns (Dummy :type Boolean))
  (bind (_weaponinfo_weaponname _weaponinfo_weapontype) (break `/Game/CombatSystem/BluePrints/Structures/S_WeaponInfo` (`/Game/CombatSystem/BluePrints/Core/Item/Weapon/BP_WeaponMaster.WeaponInfo` (`self.WeaponRef`))))
  (`self.PlaySound` (`self.GetImpactSound` _weaponinfo_weapontype) (`self.K2_GetActorLocation`))
  (`self.PlayAnimMontage` "/Game/CombatSystem/BluePrints/Player/GreatSwordAinm/Montages/Block/GreatSword_Impact.GreatSword_Impact" 1.2)
  (return false))

(fn `IsAlive`
  (returns (`Death?` :type Boolean))
  (return (`self.Dead`)))

(fn `OnDeSelected`
  (returns (Dummy :type Boolean))
  (`self.SetAllWidgets` false)
  (return false))

(fn `OnHit`
  (params (Hit_Result :type "HitResult Structure"))
  (bind (_bblockinghit _binitialoverlap _time _distance _location _impactpoint _normal _impactnormal _physmat _hitactor _hitcomponent _hitbonename) (`GameplayStatics.BreakHitResult` Hit_Result))
  (bind _asplayer (cast `/Game/CombatSystem/BluePrints/Player/Player` _hitactor))
  (`/Game/CombatSystem/BluePrints/UserInterface/BPI_CanbeAttackable.HitHandle` _asplayer self (`self.GetDamage`) (`/Game/CombatSystem/BluePrints/FunctionLibrary/BPF_CombatBaseLibrary.CalculateHitDirection` self _asplayer) (`.WeaponType_29_34EA040D45CE8853B8FEC6A08C8B7672` (break `/Game/CombatSystem/BluePrints/Structures/S_WeaponInfo` (`/Game/CombatSystem/BluePrints/Core/Item/Weapon/BP_WeaponMaster.WeaponInfo` (`self.WeaponRef`)))) (`self.GetAttackType`) _impactpoint _hitbonename))

(fn `OnSelected`
  (returns (Dummy :type Boolean))
  (`self.SetAllWidgets` true)
  (return false))

(fn `PlaySound`
  (params (SoundType :type "SoundBase Object Reference") (Location :type "Vector Structure"))
  (`GameplayStatics.PlaySoundAtLocation` SoundType Location (struct) 1.0 1.0 0.0 null null null))

(fn `RotateToTargetSmoothing`
  (params (InterpSpeed :type "Float (double-precision)"))
  (bind (_returnvalue_roll _returnvalue_pitch _returnvalue_yaw) (`KismetMathLibrary.BreakRotator` (`KismetMathLibrary.RInterpTo` (`self.K2_GetActorRotation`) (`KismetMathLibrary.FindLookAtRotation` (`self.K2_GetActorLocation`) (`self.K2_GetActorLocation` (`self.TargetRef`))) (`GameplayStatics.GetWorldDeltaSeconds`) InterpSpeed)))
  (`/Engine/EditorBlueprintResources/StandardMacros.IsValid` (`self.TargetRef`)
    (:`Is Valid`
      (`self.K2_SetActorRotation` (`KismetMathLibrary.MakeRotator` 0.0 0.0 _returnvalue_yaw))
      (return))))

(fn `Set Widget Visibility`
  (params (Widget :type "SceneComponent Object Reference") (Visibility :type Boolean))
  (`SceneComponent.SetVisibility` Widget Visibility false))

(fn `SetAllWidgets`
  (params (Visibility :type Boolean))
  (`SceneComponent.SetVisibility` (`self.HealthWidget`) Visibility false)
  (`SceneComponent.SetVisibility` (`self.TargetWidget`) Visibility false))

(fn `SetMovementSpeed`
  (params (MovementMode :type "/Game/CombatSystem/BluePrints/Enumerations/Character/E_MovementMode Enum" :default "NewEnumerator0"))
  (bind _aicontroller (`self.AIController`))
  (set `CharacterMovementComponent.MaxWalkSpeed` (select `/Game/CombatSystem/BluePrints/Enumerations/Character/E_MovementMode` MovementMode :`NewEnumerator1` (`self.WalkSpeed`) :`NewEnumerator3` (`self.JogSpeed`) :`NewEnumerator2` (`self.SprintSpeed`)) (`self.CharacterMovement`))
  (`/Game/CombatSystem/BluePrints/Enemy/AIC_EnemyController.SetEnumInBlackboard` _aicontroller (`/Game/CombatSystem/BluePrints/Enemy/AIC_EnemyController.GetMovementModeKey` _aicontroller) (enumliteral `/Game/CombatSystem/BluePrints/Enumerations/Character/E_MovementMode` MovementMode))
  (return))

(fn `SetTargetOnPerception`
  (params (TargetRef :type "Actor Object Reference"))
  (locals (LocalTargetRef :type "Actor Object Reference"))
  (bind _aicontroller (`self.AIController`))
  (set `self.TargetRef` TargetRef)
  (if (and (not (`self.InExecution`)) (`KismetSystemLibrary.IsValid` (`AIBlueprintHelperLibrary.GetBlackboard` (`self.AIController`))))
    (`/Game/CombatSystem/BluePrints/Enemy/AIC_EnemyController.SetTargetInBlackboard` _aicontroller (`self.TargetRef`))
    (`/Game/CombatSystem/BluePrints/Enemy/AIC_EnemyController.SetEnumInBlackboard` _aicontroller (`/Game/CombatSystem/BluePrints/Enemy/AIC_EnemyController.GetAIStateKey` _aicontroller) (enumliteral `/Game/CombatSystem/BluePrints/Enumerations/AI/E_AIState` "NewEnumerator1"))
    (`self.Set Widget Visibility` (`self.HealthWidget`) true)))

(fn `SimulateRigdoll`
  (returns (Dumy :type Boolean))
  (bind _aicontroller (`self.AIController`))
  (bind _mesh (`self.Mesh`))
  (bind _righthand (`self.RightHand`))
  ;[1 1 1] 设置黑板中的Enum为Dead
  (`/Game/CombatSystem/BluePrints/Enemy/AIC_EnemyController.SetEnumInBlackboard` _aicontroller (`/Game/CombatSystem/BluePrints/Enemy/AIC_EnemyController.GetAIStateKey` _aicontroller) (enumliteral `/Game/CombatSystem/BluePrints/Enumerations/AI/E_AIState` "NewEnumerator4"))
  ;[1 1 1] Set Movement
  (`CharacterMovementComponent.DisableMovement` (`self.CharacterMovement`))
  ;[1 1 1] StopBehaviorTree
  (`BrainComponent.StopLogic` (`AIController.BrainComponent` (`self.AIController`)) "")
  ;[1 1 1] 脱离控制
  (`Controller.UnPossess` (`self.AIController`))
  (`PrimitiveComponent.SetCollisionEnabled` (`self.CapsuleComponent`) "NoCollision")
  (`PrimitiveComponent.SetCollisionResponseToChannel` (`self.Mesh`) "ECC_Pawn" "ECR_Ignore")
  (`PrimitiveComponent.SetCollisionEnabled` _mesh "QueryAndPhysics")
  (`PrimitiveComponent.SetCollisionProfileName` _mesh "rigdoll" true)
  (`SkeletalMeshComponent.SetAllBodiesBelowSimulatePhysics` _mesh "pelvis" true true)
  (if (`KismetSystemLibrary.IsValid` _righthand)
    (`PrimitiveComponent.SetSimulatePhysics` _righthand true)
    (`PrimitiveComponent.SetCollisionEnabled` _righthand "QueryAndPhysics")
    (if (<= (`/Game/CombatSystem/BluePrints/Components/BPC_StatsManager.CurrentValue` (`self.BPC_Health`)) 0.0)
      (`self.Death` false))
    (return false)))

(fn `SpawnEmitter`
  (params (EmitterTemplate :type "ParticleSystem Object Reference") (Location :type "Vector Structure") (Rotation :type "Rotator Structure") (Scale :type "Vector Structure"))
  (`GameplayStatics.SpawnEmitterAtLocation` EmitterTemplate Location Rotation Scale))

(fn `Stun`
  (params (HitDirection :type "/Game/CombatSystem/BluePrints/Enumerations/Character/E_HitDirection Enum" :default "NewEnumerator3") (HitLocation :type "Vector Structure") (AttackType :type "/Game/CombatSystem/BluePrints/Enumerations/Character/E_AttackType Enum" :default "NewEnumerator4") (WeaponType :type "/Game/CombatSystem/BluePrints/Enumerations/Character/E_WeaponType Enum" :default "NewEnumerator3"))
  (bind (_stunmontage _getsucees_) (`self.GetStunMontage` HitDirection AttackType))
  (if _getsucees_
    (`self.SpawnEmitter` "/Game/CombatSystem/FPX/Weapon_Impacts/Systems/Blood/Blood_Impact_Directional_03.Blood_Impact_Directional_03" HitLocation (struct) (select `/Game/CombatSystem/BluePrints/Enumerations/Character/E_WeaponType` WeaponType :`NewEnumerator4` (2.0 2.0 2.0) :`NewEnumerator7` (1.0 1.0 1.0) :!type "Vector Structure"))
    (`AnimInstance.Montage_Play` (`self.EnemyAnimRef`) _stunmontage 1.0 "MontageLength" 0.0 true)
    (return)
    (else
      (`KismetSystemLibrary.PrintString` "敌人获取Stun动画失败"))))

(fn `UserConstructionScript`
  (bind _returnvalue (`|GetDataTableRow` "/Game/CombatSystem/BluePrints/DataTables/DT_StatInfo.DT_StatInfo" "BaseAI")
    (:`then`
      (set `self.AIStat` _returnvalue))))