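; Boss A's sword skill projectile, which damages the Player on contact and explodes, with its speed set from InitialSpeed in the construction script.
; It explodes and destroys itself shortly after a player hit, immediately on other non-enemy overlaps, or after a two-second lifetime.
; The shared Explosion event enables a blast collision that deals player damage through HitHandle and plays sound, particles and camera shake.
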(event `Explosion`
  (params (Location :type "Vector Structure"))
  (`PrimitiveComponent.SetCollisionEnabled` (`self.ExplosionCollision`) "QueryAndPhysics")
  (`GameplayStatics.PlaySoundAtLocation` "/Game/CombatSystem/AudioSystem/Explosion/Cue/Cue_Explosion_Ground_Big_01.Cue_Explosion_Ground_Big_01" (0.0 0.0 0.0) (struct) 1.0 1.0 0.0 null null null)
  (`GameplayStatics.SpawnEmitterAtLocation` "/Game/CombatSystem/ParticleSystem/Explosion/PS_Explosion_Air_Big_01.PS_Explosion_Air_Big_01" Location (struct) (3.0 3.0 3.0))
  (`PlayerCameraManager.StartMatineeCameraShake` :`self` (`GameplayStatics.GetPlayerCameraManager` 0) :`ShakeClass` "/Game/CombatSystem/BluePrints/CameraShakes/Camerashake_ExplosionShake.Camerashake_ExplosionShake_C")
  (`KismetSystemLibrary.Delay` 1.0)
  (`PrimitiveComponent.SetCollisionEnabled` (`self.ExplosionCollision`) "NoCollision"))

(event `self.ExplosionCollision.OnComponentBeginOverlap`
  (params (OverlappedComponent :type "PrimitiveComponent Object Reference") (OtherActor :type "Actor Object Reference") (OtherComp :type "PrimitiveComponent Object Reference") (OtherBodyIndex :type Integer) (bFromSweep :type Boolean) (SweepResult :type "HitResult Structure (by ref)"))
  (bind _asplayer (cast `/Game/CombatSystem/BluePrints/Player/Player` OtherActor))
  (`/Game/CombatSystem/BluePrints/UserInterface/BPI_CanbeAttackable.HitHandle` _asplayer null (`self.BaseDamage`) "NewEnumerator3" "NewEnumerator3" "NewEnumerator2" (`self.K2_GetActorLocation` _asplayer) "None"))

(event `self.ReceiveBeginPlay`
  (`KismetSystemLibrary.Delay` 2.0)
  (`self.Explosion` (`SceneComponent.K2_GetComponentLocation` (`self.SkillCollision`)))
  (`self.K2_DestroyActor`))

(event `self.SkillCollision.OnComponentBeginOverlap`
  (params (OverlappedComponent :type "PrimitiveComponent Object Reference") (OtherActor :type "Actor Object Reference") (OtherComp :type "PrimitiveComponent Object Reference") (OtherBodyIndex :type Integer) (bFromSweep :type Boolean) (SweepResult :type "HitResult Structure (by ref)"))
  (bind _asplayer (cast `/Game/CombatSystem/BluePrints/Player/Player` OtherActor)
    (:`then`
      (`/Game/CombatSystem/BluePrints/UserInterface/BPI_CanbeAttackable.HitHandle` _asplayer null (`self.BaseDamage`) "NewEnumerator3" "NewEnumerator8" "NewEnumerator1" (`self.K2_GetActorLocation` _asplayer) "None")
      (`KismetSystemLibrary.Delay` 0.2)
      (`self.Explosion` (`SceneComponent.K2_GetComponentLocation` (`self.SkillCollision`)))
      (`self.K2_DestroyActor`))
    (:`CastFailed`
      (cast `/Game/CombatSystem/BluePrints/Enemy/Enemy_Base` OtherActor
        (:`CastFailed`
          (`KismetSystemLibrary.PrintString` "OverlapWall")
          (`self.Explosion` (`SceneComponent.K2_GetComponentLocation` (`self.SwordWindow`)))
          (`self.K2_DestroyActor`))))))

(fn `UserConstructionScript`
  (set `ProjectileMovementComponent.InitialSpeed` (`self.Initial Speed`) (`self.ProjectileMovement`)))