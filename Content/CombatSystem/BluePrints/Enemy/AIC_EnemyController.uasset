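; AI controller for Enemy_Base pawns that runs the enemy's behavior tree and manages perception of the player.
; Successful sensing that passes the alive-message checks stores the target, notifies the enemy and clears the forget timer; otherwise a looping timer schedules ResetPerception.
; ResetPerception hides enemy widgets and resets blackboard AI state, target and patrol behavior, varying patrol by whether a target existed.
; Helpers expose blackboard key names and setters.
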(event `self.ReceiveBeginPlay`
  (bind _asenemy_base (cast `/Game/CombatSystem/BluePrints/Enemy/Enemy_Base` (`self.K2_GetPawn`)))
  (bind _output_get (set `self.EnemyRef` _asenemy_base))
  (bind _behaviortree (`/Game/CombatSystem/BluePrints/Enemy/Enemy_Base.BehaviorTree` _output_get))
  (`/Engine/EditorBlueprintResources/StandardMacros.IsValid` _behaviortree
    (:`Is Valid`
      (`self.RunBehaviorTree` _behaviortree)
      (`self.ResetPerception`))))

(event `self.AIPerception.OnTargetPerceptionUpdated`
  (params (Actor :type "Actor Object Reference") (Stimulus :type "AIStimulus Structure"))
  (bind _enemyref (`self.EnemyRef`))
  (if (`KismetSystemLibrary.IsValid` _enemyref)
    (bind _death_ (`/Game/CombatSystem/BluePrints/Enemy/Enemy_Base.IsAlive` _enemyref))
    (if (not _death_)
      (bind _asplayer (cast `/Game/CombatSystem/BluePrints/Player/Player` Actor))
      (bind _death__2 (message `/Game/CombatSystem/BluePrints/UserInterface/BPI_CanbeAttackable.IsAlive` _asplayer))
      (if (and (not _death__2) (`.bSuccessfullySensed` (break `AIStimulus` Stimulus)))
        (set `self.PerceptionTarget` Actor)
        (`KismetSystemLibrary.K2_ClearAndInvalidateTimerHandle` (`self.PerceptTargetTimer`))
        (`/Game/CombatSystem/BluePrints/Enemy/Enemy_Base.SetTargetOnPerception` (`self.EnemyRef`) (`self.PerceptionTarget`))
        (else
          (bind _returnvalue (`KismetSystemLibrary.K2_SetTimer` null "ResetPerception" (`self.PerceptionTime`) true))
          (set `self.PerceptTargetTimer` _returnvalue))))))

(fn `GetAICombatBehaviorKey`
  (returns (AICombatBeheviorKey :type Name))
  (return (`self.AICombatBehaviorKey`)))

(fn `GetAIHealthStateKey`
  (returns (AIHealthStateKey :type Name))
  (return (`self.AIHealthStateKey`)))

(fn `GetAIPatrolBehaviorKey`
  (returns (AIPatrolBeheviorKey :type Name))
  (return (`self.AIPatrolBehaviorKey`)))

(fn `GetAIStateKey`
  (returns (AIStateKey :type Name))
  (return (`self.AIStateKey`)))

(fn `GetAttackTypeKey`
  (returns (AttackTypeKey :type Name))
  (return (`self.AttackTypeKey`)))

(fn `GetLastFindTargetLocationKey`
  (returns (LastFindTargetLocationKey :type Name))
  (return (`self.LastFindTargetLocationKey`)))

(fn `GetMovementModeKey`
  (returns (MovementModeKey :type Name))
  (return (`self.MovementModeKey`)))

(fn `GetRangeToTargetKey`
  (returns (RangeToTargetKey :type Name))
  (return (`self.RangeToTargetKey`)))

(fn `GetRotationModeKey`
  (returns (RotationModeKey :type Name))
  (return (`self.RotationModeKey`)))

(fn `GetTargetKey`
  (returns (TargetKey :type Name))
  (return (`self.TargetKey`)))

(fn `ResetPerception`
  (if (and (`KismetSystemLibrary.IsValid` (`self.Blackboard`)) (`KismetSystemLibrary.IsValid` (`self.EnemyRef`)))
    (`/Engine/EditorBlueprintResources/StandardMacros.IsValid` (`self.PerceptionTarget`)
      (:`Is Valid`
        (`/Game/CombatSystem/BluePrints/Enemy/Enemy_Base.SetAllWidgets` (`self.EnemyRef`) false)
        (set `self.PerceptionTarget` null)
        (`BlackboardComponent.SetValueAsEnum` (`self.Blackboard`) (`self.GetAIStateKey`) (enumliteral `/Game/CombatSystem/BluePrints/Enumerations/AI/E_AIState` "NewEnumerator0"))
        (`BlackboardComponent.SetValueAsObject` (`self.Blackboard`) (`self.GetTargetKey`) (`self.PerceptionTarget`))
        (`BlackboardComponent.SetValueAsEnum` (`self.Blackboard`) (`self.AIPatrolBehaviorKey`) (enumliteral `/Game/CombatSystem/BluePrints/Enumerations/AI/E_AIPatrolBehavior` "NewEnumerator2")))
      (:`Is Not Valid`
        (`/Game/CombatSystem/BluePrints/Enemy/Enemy_Base.SetAllWidgets` (`self.EnemyRef`) false)
        (`BlackboardComponent.SetValueAsEnum` (`self.Blackboard`) (`self.GetAIStateKey`) (enumliteral `/Game/CombatSystem/BluePrints/Enumerations/AI/E_AIState` "NewEnumerator0"))
        (`BlackboardComponent.SetValueAsObject` (`self.Blackboard`) (`self.GetTargetKey`) (`self.PerceptionTarget`))
        (`BlackboardComponent.SetValueAsEnum` (`self.Blackboard`) (`self.AIPatrolBehaviorKey`) (enumliteral `/Game/CombatSystem/BluePrints/Enumerations/AI/E_AIPatrolBehavior` "NewEnumerator0"))))))

(fn `SetEnumInBlackboard`
  (params (KeyName :type "Name (by ref)") (EnumValue :type Byte))
  (if (`KismetSystemLibrary.IsValid` (`self.Blackboard`))
    (`BlackboardComponent.SetValueAsEnum` (`self.Blackboard`) KeyName EnumValue)))

(fn `SetTargetInBlackboard`
  (params (TargetRef :type "Actor Object Reference"))
  (`/Engine/EditorBlueprintResources/StandardMacros.IsValid` (`self.Blackboard`)
    (:`Is Valid`
      (`BlackboardComponent.SetValueAsObject` (`self.Blackboard`) (`self.GetTargetKey`) TargetRef))
    (:`Is Not Valid`
      (`KismetSystemLibrary.PrintString` "BlackBoardIsNotValid"))))

(fn `UserConstructionScript`)