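; Animation notify that spawns a boss skill actor at a chosen moment in an Enemy_BossA animation.
; It casts the mesh owner to Enemy_BossA and places the configurable skill class relative to the boss's DirectionArrow, using up and forward offsets, the arrow's rotation and a configurable scale.
; The spawned skill is owned by the boss; other owners are ignored and the notify returns false.
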(fn `Received_Notify`
  (params (MeshComp :type "SkeletalMeshComponent Object Reference") (Animation :type "AnimSequenceBase Object Reference"))
  (returns (ReturnValue :type Boolean))
  (bind _asenemy_boss_a (cast `/Game/CombatSystem/BluePrints/Enemy/Boss/BossA/Enemy_BossA` (`ActorComponent.GetOwner` MeshComp))
    (:`then`
      (bind _directionarrow (`/Game/CombatSystem/BluePrints/Enemy/Boss/BossA/Enemy_BossA.DirectionArrow` _asenemy_boss_a))
      (`|SpawnActorFromClass` (`self.Skill Class`) (`KismetMathLibrary.MakeTransform` (+ (.location (`SceneComponent.K2_GetComponentToWorld` _directionarrow)) (* (`SceneComponent.GetUpVector` _directionarrow) (`self.SkillUpLength`)) (* (`SceneComponent.GetForwardVector` _directionarrow) (`self.SkillForwardLength`))) (.rotation (`SceneComponent.K2_GetComponentToWorld` _directionarrow)) (`self.SkillScal`)) "Undefined" "OverrideRootScale" _asenemy_boss_a null)
      (return true))
    (:`CastFailed`
      (return false))))