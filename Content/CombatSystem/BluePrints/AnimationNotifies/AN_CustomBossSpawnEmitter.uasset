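; Anim notify that spawns the ground-hit particle effect for Enemy_BossA during an animation.
; It casts the mesh owner to the boss and attaches its HitGroundPartical emitter to the mesh at the GreatSwordTrailEnd point.
; The emitter scale follows the health state enum read from the AI controller's Blackboard, enlarged only in the High state.
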(fn `Received_Notify`
  (params (MeshComp :type "SkeletalMeshComponent Object Reference") (Animation :type "AnimSequenceBase Object Reference"))
  (returns (ReturnValue :type Boolean))
  (bind _asenemy_boss_a (cast `/Game/CombatSystem/BluePrints/Enemy/Boss/BossA/Enemy_BossA` (`ActorComponent.GetOwner` MeshComp)))
  (bind _aicontroller (`/Game/CombatSystem/BluePrints/Enemy/Enemy_Base.AIController` _asenemy_boss_a))
  (`GameplayStatics.SpawnEmitterAttached` (`/Game/CombatSystem/BluePrints/Enemy/Boss/BossA/Enemy_BossA.HitGroundPartical` _asenemy_boss_a) (`Character.Mesh` _asenemy_boss_a) "GreatSwordTrailEnd" (0.0 0.0 0.0) (struct) (select `/Game/CombatSystem/BluePrints/Enumerations/AI/E_HealthState` (enumliteral `/Game/CombatSystem/BluePrints/Enumerations/AI/E_HealthState` (cast `/Game/CombatSystem/BluePrints/Enumerations/AI/E_HealthState` (`BlackboardComponent.GetValueAsEnum` (`AIBlueprintHelperLibrary.GetBlackboard` _aicontroller) (`/Game/CombatSystem/BluePrints/Enemy/AIC_EnemyController.GetAIHealthStateKey` _aicontroller)))) :`NewEnumerator0` (1.0 1.0 1.0) :`NewEnumerator1` (1.0 1.0 1.0) :`NewEnumerator2` (1.0 1.0 1.0) :`NewEnumerator3` (3.0 3.0 3.0) :!type "Vector Structure"))
  (return true))