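; Player lock-on component that finds, tracks and cycles targets implementing BPI_IsTargetable.
; Targets are filtered by range, screen position, line of sight and death; opening picks the nearest, or resets the camera if none.
; An angle-sorted map drives wrap-around left/right switching.
; Tick interpolates control rotation toward the target and releases after prolonged occlusion or death, with character rotation mode swapped during lock and restored on close.
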(event `InitialVariable`
  (bind (_asplayer _bsuccess) (cast `/Game/CombatSystem/BluePrints/Player/Player` (`self.GetOwner`) :!pure true))
  ;[0 0 0] Initial
  (if _bsuccess
    (bind _output_get (set `self.OwnerRef` _asplayer))
    (set `self.OwnerCamera` (`/Game/CombatSystem/BluePrints/Player/Player.Camera` _output_get))
    (`self.SaveOwnerRotationMode`)))

(event `self.ReceiveBeginPlay`
  ;[0.1039 1 0] BeginPlay
  (`self.InitialVariable`))

(event `OpenTargetSystem`
  ;[0.09375 0.09375 0.09375] Open
  (set `self.TargetingOpen?` true)
  (bind (_hastarget_ _targetmapvals) (`self.FindTarget`))
  (if _hastarget_
    (bind _output_get (set `self.TargetsMap` _targetmapvals))
    ;;[0.6302 0.6302 0.6302] 获取距离最近的Enemy
    (bind _keys (`BlueprintMapLibrary.Map_Keys` _output_get))
    (set `self.CurrentTarget` (`|GetArrayItem` _keys (`KismetMathLibrary.MinOfFloatArray` (`self.DistanceArray`))))
    (`self.SortTargetMap`)
    (`self.SetOwnerRotationMode` "NewEnumerator0")
    (else
      (`self.CloseTargetSystem`)
      ;;[1 1 1] 当没有敌人的时候索敌的话就切换视角到当前人物的朝向
      (`self.SetCameraReverse`))))

(event `CloseTargetSystem`
  ;[0.09375 0.09375 0.09375] Close
  (`self.DisableCameraLock`)
  (`self.SetOwnerRotationMode` "NewEnumerator7")
  (set `self.CurrentTarget` null))

(event `self.ReceiveTick`
  (params (DeltaSeconds :type "Float (single-precision)"))
  (bind (_target _hitanyblock_) (`self.SightOfLineCheck` (`self.CurrentTarget`)))
  ;[1 0.8475 0] Event Tick
  (bind _death_ (`/Game/CombatSystem/BluePrints/Player/Player.IsAlive` (`self.OwnerRef`)))
  (if (not _death_)
    (`self.Enable Camera Lock`)
    (`|ExecutionSequence`
      (:`then_0`
        (if (`self.IsTargetingEnable?`)
          ;;[1 1 1] 锁定视角后当Target被挡住后多久取消锁定
          (if _hitanyblock_
            (`/Engine/EditorBlueprintResources/StandardMacros.DoOnce` false :!label _label
              (:`Completed`
                (bind _output_get (set `self.RecordTarget` _target))
                (`KismetSystemLibrary.RetriggerableDelay` (`self.KeepingTargetTime`))
                (set `self.CurrentTarget` _output_get)
                (`self.CloseTargetSystem`)))
            (else
              (`|ExecutionSequence`
                (:`then_0`
                  (goto _label :!via `Reset`))
                (:`then_1`
                  (set `self.RecordTarget` (`self.RecordTarget`))
                  (`self.Enable Camera Lock`)
                  (set `self.RecordTarget` null)))))))
      (:`then_1`
        (if (`self.Target Is Death?` (`self.CurrentTarget`))
          (`self.CloseTargetSystem`)))
      (:`then_2`
        (goto _label_2 :!via `Reset`)))
    (else
      (`/Engine/EditorBlueprintResources/StandardMacros.DoOnce` false :!label _label_2
        (:`Completed`
          (`self.CloseTargetSystem`))))))

(fn `ChangeTarget`
  (params (`ChangeLeft?` :type Boolean))
  (locals (ChangeVals :type Boolean) (LocalMaxMapIndex :type Integer :default 0))
  (set `local.ChangeVals` `ChangeLeft?`)
  (set `self.TargetingOpen?` true)
  (bind (_hastarget_ _targetmapvals) (`self.FindTarget`))
  (bind _output_get (set `self.TargetsMap` _targetmapvals))
  (`self.SortTargetMap`)
  (bind _returnvalue (`BlueprintMapLibrary.Map_Length` _output_get))
  (set `local.LocalMaxMapIndex` (- _returnvalue 1))
  (if (> _returnvalue 1)
    (if (`local.ChangeVals`)
      (if (== (`self.CheckCurrentIndexInMap`) 0)
        (bind _keys (`BlueprintMapLibrary.Map_Keys` (`self.TargetsMap`)))
        (`self.DisableCameraLock`) ; 取消当前锁定
        (set `self.CurrentTarget` (`|GetArrayItem` _keys (`local.LocalMaxMapIndex`)))
        ;[1 1 1] 切换新的锁定
        (`self.Enable Camera Lock`)
        (`self.UpdateCameraRotation`)
        (else
          (bind _keys_2 (`BlueprintMapLibrary.Map_Keys` (`self.TargetsMap`)))
          (bind _keys_3 (`BlueprintMapLibrary.Map_Keys` (`self.TargetsMap`)))
          (`self.DisableCameraLock`)
          (set `self.CurrentTarget` (`|GetArrayItem` _keys_3 (- (`KismetArrayLibrary.Array_Find` _keys_2 (`self.CurrentTarget`)) 1)))
          (`self.Enable Camera Lock`)
          (`self.UpdateCameraRotation`)))
      (elif (== (`self.CheckCurrentIndexInMap`) (`local.LocalMaxMapIndex`))
        (bind _keys_4 (`BlueprintMapLibrary.Map_Keys` (`self.TargetsMap`)))
        (`self.DisableCameraLock`)
        (set `self.CurrentTarget` (`|GetArrayItem` _keys_4))
        (`self.Enable Camera Lock`)
        (`self.UpdateCameraRotation`)
        (else
          (bind _keys_5 (`BlueprintMapLibrary.Map_Keys` (`self.TargetsMap`)))
          (bind _keys_6 (`BlueprintMapLibrary.Map_Keys` (`self.TargetsMap`)))
          (`self.DisableCameraLock`)
          (set `self.CurrentTarget` (`|GetArrayItem` _keys_6 (+ (`KismetArrayLibrary.Array_Find` _keys_5 (`self.CurrentTarget`)) 1)))
          (`self.Enable Camera Lock`)
          (`self.UpdateCameraRotation`))))
    (return)))

(fn `CheckCurrentIndexInMap`
  (returns (CurrentIndex :type Integer))
  (bind _keys (`BlueprintMapLibrary.Map_Keys` (`self.TargetsMap`)))
  (return (`KismetArrayLibrary.Array_Find` _keys (`self.CurrentTarget`))))

(fn `DisableCameraLock`
  (bind _currenttarget (`self.CurrentTarget`))
  (`/Engine/EditorBlueprintResources/StandardMacros.IsValid` _currenttarget
    (:`Is Valid`
      (message `/Game/CombatSystem/BluePrints/UserInterface/BPI_IsTargetable.OnDeSelected` _currenttarget))
    (:`Is Not Valid`
      _))
  (set `self.TargetingOpen?` false))

(fn `Enable Camera Lock`
  (set `self.TargetingOpen?` true)
  (`self.UpdateCameraRotation`)
  (message `/Game/CombatSystem/BluePrints/UserInterface/BPI_IsTargetable.OnSelected` (`self.CurrentTarget`)))

(fn `FindTarget`
  (returns (`HasTarget?` :type Boolean) (TargetMapVals :type "Map of Actor Object Reference to Float (double-precision)"))
  (locals (LocalTarget :type "Actor Object Reference") (LocalTargetMap :type "Map of Actor Object Reference to Float (double-precision)"))
  (`BlueprintMapLibrary.Map_Clear` (`self.TargetsMap`))
  (`KismetArrayLibrary.Array_Clear` (`self.DistanceArray`))
  (bind _outactors (`GameplayStatics.GetAllActorsWithInterface` "/Game/CombatSystem/BluePrints/UserInterface/BPI_IsTargetable.BPI_IsTargetable_C"))
  (for _array_element _outactors
    (bind (_target _hitanyblock_) (`self.SightOfLineCheck` _array_element))
    (if (and (`KismetSystemLibrary.IsValid` _target) (<= (`self.GetDistanceToTarget` _array_element) (`self.MaxDistanceCanSeeTarget`)) (`self.IsInViewportCheck` _array_element) (not _hitanyblock_) (not (`self.Target Is Death?` _array_element)))
      (bind _output_get (set `local.LocalTarget` _target))
      (bind _yawrotation (`self.CulculateDeltaRotation` _target))
      (`BlueprintMapLibrary.Map_Add` (`local.LocalTargetMap`) _output_get _yawrotation)
      (`KismetArrayLibrary.Array_Add` (`self.DistanceArray`) (`self.GetDistanceToTarget` _output_get))
      ;[1 1 1] Debug Rotation Test
      (`KismetSystemLibrary.PrintString` (`KismetStringLibrary.Concat_StrStr` (`KismetSystemLibrary.GetDisplayName` (`local.LocalTarget`)) "的角度: " (`KismetStringLibrary.Conv_DoubleToString` _yawrotation)))))
  (if (> (`BlueprintMapLibrary.Map_Length` (`local.LocalTargetMap`)) 0)
    (`self.SetOwnerRotationMode` "NewEnumerator0")
    (return true (`local.LocalTargetMap`))
    (else
      (return false))))

(fn `IsInViewportCheck`
  (params (Target :type "Actor Object Reference"))
  (returns (`InViewport?` :type Boolean))
  (bind (_screenposition _returnvalue) (`self.GetPositionOnScreen` Target))
  (bind _returnvalue_2 (and (`self.IsInViewPort?` _screenposition) _returnvalue))
  (if _returnvalue_2
    (return _returnvalue_2)
    (else
      (`KismetSystemLibrary.PrintString` (`KismetStringLibrary.Concat_StrStr` (`KismetSystemLibrary.GetDisplayName` Target) "不在屏幕中无法被检测到")))))

(fn `IsTargetingEnable?`
  (returns (`Enable?` :type Boolean))
  (return (`KismetSystemLibrary.IsValid` (`self.CurrentTarget`))))

(fn `LineTraceStart`
  (returns (Start :type "Vector Structure"))
  (bind _ownercamera (`self.OwnerCamera`))
  (return (+ (`SceneComponent.K2_GetComponentLocation` _ownercamera) (* (`SceneComponent.GetForwardVector` _ownercamera) (`self.CameraDepthOffset`)) (* (`SceneComponent.GetUpVector` _ownercamera) (`self.CameraHeightOffset`)))))

(fn `SaveOwnerRotationMode`
  (bind _ownerref (`self.OwnerRef`))
  (bind _ownerref_2 (`self.OwnerRef`))
  (bind _charactermovement (`Character.CharacterMovement` _ownerref))
  (`/Engine/EditorBlueprintResources/StandardMacros.IsValid` _ownerref_2
    (:`Is Valid`
      (set `self.OwnerControllerRotationYaw` (`Pawn.bUseControllerRotationYaw` _ownerref))
      (bind _output_get (set `self.OwnerOrientRotationToMovement` (`CharacterMovementComponent.bOrientRotationToMovement` _charactermovement)))
      (set `self.OwnerControllerDesiredRotation` (`CharacterMovementComponent.bUseControllerDesiredRotation` _charactermovement))
      (`KismetSystemLibrary.PrintString` (`KismetStringLibrary.Conv_BoolToString` _output_get)))
    (:`Is Not Valid`
      (`KismetSystemLibrary.PrintString` (`KismetStringLibrary.Concat_StrStr` (`KismetSystemLibrary.GetDisplayName` _ownerref_2) "为空，存储RotationMode失败")))))

(fn `SetCameraReverse`
  (bind _ownerref (`self.OwnerRef`))
  (bind (_returnvalue_roll _returnvalue_pitch _returnvalue_yaw) (`KismetMathLibrary.BreakRotator` (`Actor.K2_GetActorRotation` _ownerref)))
  (`Controller.SetControlRotation` (`Pawn.GetController` _ownerref) (`KismetMathLibrary.MakeRotator` 0.0 0.0 _returnvalue_yaw))
  (return))

(fn `SetOwnerRotationMode`
  (params (RotationMode :type "/Game/CombatSystem/BluePrints/Enumerations/Character/E_RotationMode Enum" :default "NewEnumerator0"))
  (bind _ownerref (`self.OwnerRef`))
  (bind _ownerref_2 (`self.OwnerRef`))
  (bind _charactermovement (`Character.CharacterMovement` _ownerref))
  (bind _charactermovement_2 (`Character.CharacterMovement` _ownerref_2))
  (if (`self.IsTargetingEnable?`)
    (switch `/Game/CombatSystem/BluePrints/Enumerations/Character/E_RotationMode` RotationMode
      (:`NewEnumerator0`
        (set `Pawn.bUseControllerRotationYaw` false _ownerref_2)
        (set `CharacterMovementComponent.bOrientRotationToMovement` false _charactermovement_2)
        (set `CharacterMovementComponent.bUseControllerDesiredRotation` true _charactermovement_2))
      (:`NewEnumerator7`
        (set `Pawn.bUseControllerRotationYaw` (`self.OwnerControllerRotationYaw`) _ownerref)
        (set `CharacterMovementComponent.bOrientRotationToMovement` (`self.OwnerOrientRotationToMovement`) _charactermovement)
        (set `CharacterMovementComponent.bUseControllerDesiredRotation` (`self.OwnerControllerDesiredRotation`) _charactermovement)))))

(fn `SightOfLineCheck`
  (params (TargetRef :type "Actor Object Reference"))
  (returns (Target :type "Actor Object Reference") (`HItAnyBlock?` :type Boolean))
  (locals (LocalTarget :type "Actor Object Reference"))
  (bind _output_get (set `local.LocalTarget` TargetRef))
  (if (`KismetSystemLibrary.IsValid` _output_get)
    (bind (_outhit _returnvalue) (`KismetSystemLibrary.LineTraceSingleForObjects` (`self.LineTraceStart`) (`Actor.K2_GetActorLocation` (`local.LocalTarget`)) (`self.CanHitActors`) false (`|MakeArray` (`self.OwnerRef`) :!type "Actor Object Reference")))
    (`|ExecutionSequence`
      (:`then_0`
        (return (`local.LocalTarget`) _returnvalue))
      (:`then_1`
        (return null _returnvalue)))))

(fn `SortTargetMap`
  (locals (LocalMap :type "Map of Actor Object Reference to Float (double-precision)") (NewLocalVar_0 :type "Map of Actor Object Reference to Float (double-precision)"))
  (while (!= (`BlueprintMapLibrary.Map_Length` (`self.TargetsMap`)) 0)
    (bind _values (`BlueprintMapLibrary.Map_Values` (`self.TargetsMap`)))
    (bind _keys (`BlueprintMapLibrary.Map_Keys` (`self.TargetsMap`)))
    (bind (_indexofminvalue _minvalue) (`KismetMathLibrary.MinOfFloatArray` _values))
    (bind _output (`|GetArrayItem` _keys _indexofminvalue))
    (`BlueprintMapLibrary.Map_Add` (`local.LocalMap`) _output _minvalue)
    (`BlueprintMapLibrary.Map_Remove` (`self.TargetsMap`) _output))
  (set `self.TargetsMap` (`local.LocalMap`)))

(fn `Target Is Death?`
  (params (Target :type "Object Object Reference"))
  (returns (`Death?` :type Boolean))
  (bind _death_ (message `/Game/CombatSystem/BluePrints/UserInterface/BPI_CanbeAttackable.IsAlive` Target))
  (return _death_))

(fn `UpdateCameraRotation`
  (locals (ControllerRef :type "Controller Object Reference"))
  (bind _ownerref (`self.OwnerRef`))
  (bind _currenttarget (`self.CurrentTarget`))
  (bind (_returnvalue_roll _returnvalue_pitch _returnvalue_yaw) (`KismetMathLibrary.BreakRotator` (`KismetMathLibrary.FindLookAtRotation` (`Actor.K2_GetActorLocation` _ownerref) (`Actor.K2_GetActorLocation` _currenttarget))))
  (if (`KismetSystemLibrary.IsValid` _currenttarget)
    (set `local.ControllerRef` (`Pawn.GetController` _ownerref))
    (`Controller.SetControlRotation` (`local.ControllerRef`) (`KismetMathLibrary.RInterpTo` (`Controller.GetControlRotation` (`local.ControllerRef`)) (`KismetMathLibrary.MakeRotator` 0.0 (- _returnvalue_pitch 5.0) _returnvalue_yaw) (`GameplayStatics.GetWorldDeltaSeconds`) (`self.LockInterpSpeed`)))))