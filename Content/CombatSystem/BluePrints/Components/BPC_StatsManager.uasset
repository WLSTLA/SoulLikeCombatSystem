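; Stat component for the combat system that manages one clamped value, such as health or stamina, with optional regeneration and two progress bars.
; UpdateStat applies a delta, snaps the first bar, starts a delayed timer-driven interpolation of the second as a trailing bar, and reports depletion.
; Regeneration waits out a retriggerable delay, then a looping timer feeds RegenValue back through UpdateStat; interrupting changes clear that timer.
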(event `UpdateBar2 LerpEvent`
  ;[1 1 1] Bar2Update Event
  (`KismetSystemLibrary.K2_PauseTimer` null "ProgreessBar2 Lerp")
  (`KismetSystemLibrary.RetriggerableDelay` (`self.Bar2 PauseTime`))
  (`KismetSystemLibrary.K2_SetTimer` null "ProgreessBar2 Lerp" 0.1 true))

(event `InitialStats`
  (params (Progressbar1 :type "ProgressBar Object Reference") (Progressbar2 :type "ProgressBar Object Reference"))
  ;[1 1 1] Initial
  (set `self.Progressbar1` Progressbar1)
  (set `self.Progressbar2` Progressbar2)
  (`self.ResetStat`)
  (if (`self.CanRegeneration`)
    (`self.RestroyRegenSpeed`)))

(event `Regeneration Event`
  ;[1 1 1] Regeneration Event
  (if (`self.CanRegeneration`)
    (set `self.BaseInterpSpeed` 20.0)
    (if (not (`KismetSystemLibrary.K2_IsTimerActiveHandle` (`self.RegenTimer`)))
      (`KismetSystemLibrary.RetriggerableDelay` (`self.RegenPauseTime`))
      (bind _returnvalue (`KismetSystemLibrary.K2_SetTimer` null "RegenTick" (`self.RegenSpeed`) true))
      (set `self.RegenTimer` _returnvalue))))

(event `UpdateBar1 LerpEvent`
  ;[1 1 1] Bar1Update Event
  (`KismetSystemLibrary.K2_PauseTimer` null "ProgreessBar1 Lerp")
  (`KismetSystemLibrary.RetriggerableDelay` (`self.Bar1 PauseTime`))
  (`KismetSystemLibrary.K2_SetTimer` null "ProgreessBar1 Lerp" 0.1 true))

(fn `CheckCurrentValueIsEnough`
  (params (Value :type "Float (double-precision)"))
  (returns (`Enough?` :type Boolean))
  (return (<= Value (`self.CurrentValue`))))

(fn `ClearRegen`
  (bind _regentimer (`self.RegenTimer`))
  (if (`KismetSystemLibrary.K2_IsTimerActiveHandle` _regentimer)
    (`KismetSystemLibrary.K2_ClearAndInvalidateTimerHandle` _regentimer)))

(fn `CurrentValueIsEmpty?`
  (returns (`Empty?` :type Boolean))
  (return (<= (`self.CurrentValue`) (`self.MinValue`))))

(fn `ModifyRegenSpeed`
  (params (Value :type "Float (double-precision)"))
  (set `self.RegenValue` (`KismetMathLibrary.FClamp` (+ Value (`self.RegenValue`)) (`self.MinValue`) (`self.MaxValue`))))

(fn `ProgreessBar1 Lerp`
  (`/Engine/EditorBlueprintResources/StandardMacros.IsValid` (`self.Progressbar1`)
    (:`Is Valid`
      (if (`KismetMathLibrary.NearlyEqual_FloatFloat` (`KismetMathLibrary.FInterpTo` (`ProgressBar.Percent` (`self.Progressbar1`)) (`self.GetPercentage`) (`GameplayStatics.GetWorldDeltaSeconds`) (`self.CalculateInterpMulitiplies`)) (`self.CurrentValue`) 0.0001)
        (`KismetSystemLibrary.K2_PauseTimer` null "ProgreessBar1 Lerp")
        (else
          (`self.ProgreessBar1 Update` (`KismetMathLibrary.FInterpTo` (`ProgressBar.Percent` (`self.Progressbar1`)) (`self.GetPercentage`) (`GameplayStatics.GetWorldDeltaSeconds`) (`self.CalculateInterpMulitiplies`)))))
      (return))
    (:`Is Not Valid`
      (`KismetSystemLibrary.K2_PauseTimer` null "ProgreessBar1 Lerp"))))

(fn `ProgreessBar1 Update`
  (params (InPercent :type "Float (double-precision)"))
  (`/Engine/EditorBlueprintResources/StandardMacros.IsValid` (`self.Progressbar1`)
    (:`Is Valid`
      (`ProgressBar.SetPercent` (`self.Progressbar1`) InPercent)
      (return))))

(fn `ProgreessBar2 Lerp`
  (`/Engine/EditorBlueprintResources/StandardMacros.IsValid` (`self.Progressbar2`)
    (:`Is Valid`
      (if (`KismetMathLibrary.NearlyEqual_FloatFloat` (`KismetMathLibrary.FInterpTo` (`ProgressBar.Percent` (`self.Progressbar2`)) (`self.GetPercentage`) (`GameplayStatics.GetWorldDeltaSeconds`) (`self.CalculateInterpMulitiplies`)) (`self.CurrentValue`) 0.0001)
        (`KismetSystemLibrary.K2_PauseTimer` null "ProgreessBar2 Lerp")
        (else
          (`self.ProgreessBar2 Update` (`KismetMathLibrary.FInterpTo` (`ProgressBar.Percent` (`self.Progressbar2`)) (`self.GetPercentage`) (`GameplayStatics.GetWorldDeltaSeconds`) (`self.CalculateInterpMulitiplies`)))))
      (return))
    (:`Is Not Valid`
      (`KismetSystemLibrary.K2_PauseTimer` null "ProgreessBar2 Lerp"))))

(fn `ProgreessBar2 Update`
  (params (InPercent :type "Float (double-precision)"))
  (`/Engine/EditorBlueprintResources/StandardMacros.IsValid` (`self.Progressbar2`)
    (:`Is Valid`
      (`ProgressBar.SetPercent` (`self.Progressbar2`) InPercent))))

(fn `RegenTick`
  (`self.Update Stat` (`self.RegenValue`))
  (return))

(fn `ResetStat`
  (`self.SetCurrentValue` (`self.MaxValue`)
    (:`Out`
      (`self.UpdateBar1 LerpEvent`)
      (`self.UpdateBar2 LerpEvent`))))

(fn `RestroyRegenSpeed`
  (set `self.RegenValue` (`self.OriginalRegenValue`)))

(fn `Update Stat`
  (params (Value :type "Float (double-precision)") (`CanInterruptRegan?` :type Boolean))
  (returns (`IsValueEmpty?` :type Boolean))
  (locals (LocalValue :type "Float (double-precision)"))
  (if `CanInterruptRegan?`
    (`self.ClearRegen`))
  (bind _currentvalue (`self.SetCurrentValue` Value)
    (:`Out`
      (if (<= _currentvalue 0.0)
        (`self.ProgreessBar1 Update` (`self.GetPercentage`))
        (`self.UpdateBar2 LerpEvent`)
        ;[1 1 1] Regeneration If Need
        (`self.Regeneration Event`)
        (return true)
        (else
          (`self.ProgreessBar1 Update` (`self.GetPercentage`))
          (`self.UpdateBar2 LerpEvent`)
          (`self.Regeneration Event`)
          (return false))))))