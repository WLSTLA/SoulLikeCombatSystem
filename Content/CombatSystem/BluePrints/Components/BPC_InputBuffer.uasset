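; Input buffer component for the combat system that holds the latest input key while its window is open.
; UpdateBuffer overwrites the single stored key and consumes it immediately if the buffer is closed.
; Closing the buffer consumes whatever key is stored, then fires the closed event.
; Consuming broadcasts the key through the consumed event and resets it to a default enum value.
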(fn `CloseBuffer`
  (set `self.IsOpen?` false)
  (`self.ConsumeStoryKey`)
  (`self.OnInputBufferClosed`))

(fn `ConsumeStoryKey`
  (`self.OnInputBufferConsumed` (`self.StoryKey`))
  (set `self.StoryKey` "NewEnumerator6"))

(fn `OpenBuffer`
  (set `self.IsOpen?` true))

(fn `UpdateBuffer`
  (params (InputKey :type "/Game/CombatSystem/BluePrints/Enumerations/Character/E_InputKey Enum" :default "NewEnumerator0"))
  (set `self.StoryKey` InputKey)
  (if (not (`self.IsOpen?`))
    (`self.ConsumeStoryKey`)))