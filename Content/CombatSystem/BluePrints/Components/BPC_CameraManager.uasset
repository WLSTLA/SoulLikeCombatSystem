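; Player camera component that caches the owner's camera, spring arm and camera manager and provides combat feedback effects.
; It plays light or heavy camera shakes and toggles global slow motion.
; On owner death it briefly slows time and lowers audio pitch, then restores both.
; Arm length changes are eased by a looping timer running FInterpTo, which clears itself once near the target.
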(event `self.ReceiveBeginPlay`
  ;[1 1 1] Begin
  (bind _asplayer (cast `/Game/CombatSystem/BluePrints/Player/Player` (`self.GetOwner`)))
  (set `self.OwnerCamera` (`/Game/CombatSystem/BluePrints/Player/Player.Camera` _asplayer))
  (set `self.OwnerSpringArm` (`/Game/CombatSystem/BluePrints/Player/Player.SpringArm` _asplayer))
  (set `self.OwnerCameraManager` (`GameplayStatics.GetPlayerCameraManager` 0)))

(event `Play Camera Shake`
  (params (ShakeType :type "/Game/CombatSystem/BluePrints/Enumerations/Character/E_CameraShakeType Enum" :default "NewEnumerator0"))
  ;[1 1 1] Play Camera Shake
  (`PlayerCameraManager.PlayCameraShake` :`self` (`self.OwnerCameraManager`) :`ShakeClass` (select `/Game/CombatSystem/BluePrints/Enumerations/Character/E_CameraShakeType` ShakeType :`NewEnumerator0` "/Game/CombatSystem/BluePrints/CameraShakes/Camerashake_Light.Camerashake_Light_C" :`NewEnumerator1` "/Game/CombatSystem/BluePrints/CameraShakes/Camerashake_Heavy.Camerashake_Heavy_C" :!type "CameraShake Class Reference")))

(event `OpenTimeDilation`
  ;[1 1 1] Timedilation
  (`GameplayStatics.SetGlobalTimeDilation` 0.1))

(event `OwnerDeathTimeDilation`
  ;[1 1 1] 角色死亡后触发
  (`GameplayStatics.SetGlobalTimeDilation` 0.1)
  (`GameplayStatics.SetGlobalPitchModulation` 0.8)
  (`KismetSystemLibrary.Delay` 0.3)
  (`GameplayStatics.SetGlobalTimeDilation` 1.0)
  (`GameplayStatics.SetGlobalPitchModulation` 1.0))

(event `CloseTimeDilation`
  ;[1 1 1] Timedilation
  (`GameplayStatics.SetGlobalTimeDilation` 1.0))

(event `SmothingUpdateCamera`
  (params (TargetArmlength :type "Float (double-precision)"))
  ;[1 1 1] 平滑改变相机得位置
  (set `self.TargetArmLength` TargetArmlength)
  (if (not (`KismetSystemLibrary.K2_IsTimerActiveHandle` (`self.SmothingTimer`)))
    (bind _returnvalue (`KismetSystemLibrary.K2_SetTimer` null "SmothingUpdateArm" (`self.DeathCameraTick`) true))
    (set `self.SmothingTimer` _returnvalue)))

(fn `SmothingUpdateArm`
  (bind _ownerspringarm (`self.OwnerSpringArm`))
  (`/Engine/EditorBlueprintResources/StandardMacros.IsValid` _ownerspringarm
    (:`Is Valid`
      (bind _output_get (set `SpringArmComponent.TargetArmLength` (`KismetMathLibrary.FInterpTo` (`SpringArmComponent.TargetArmLength` _ownerspringarm) (`self.TargetArmLength`) (`GameplayStatics.GetWorldDeltaSeconds`) (`self.ArmInterpSpeed`)) (`self.OwnerSpringArm`)))
      (if (`KismetMathLibrary.NearlyEqual_FloatFloat` _output_get (`self.TargetArmLength`) 0.1)
        (`KismetSystemLibrary.K2_ClearAndInvalidateTimerHandle` (`self.SmothingTimer`))
        (return)))))