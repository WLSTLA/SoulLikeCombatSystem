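; Combat component that detects weapon hits by tracing the paths of the weapon mesh's sockets between frames.
; UpdateWeaponAndSocet caches the mesh and socket names, and EnableTrace and DisableTrace toggle tracing and reset the ignore list.
; While enabled, Tick line-traces from each socket's previous location to its current one, then stores the new locations.
; Hit loops break on BPI_CanbeAttackable actors, then ignore the actor and broadcast OnHit.
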(event `UpdateWeaponAndSocet`
  (params (WeaponMesh :type "StaticMeshComponent Object Reference"))
  ;[0 0 0] Setup WeaponSocket
  (`/Engine/EditorBlueprintResources/StandardMacros.IsValid` WeaponMesh
    (:`Is Valid`
      (`KismetArrayLibrary.Array_Clear` (`self.SocketName`))
      (set `self.Mesh` WeaponMesh)
      (set `self.SocketName` (`SceneComponent.GetAllSocketNames` (`self.Mesh`)))
      (`BlueprintMapLibrary.Map_Clear` (`self.PreSocketLocation`)))
    (:`Is Not Valid`
      (`KismetSystemLibrary.PrintString` (`KismetStringLibrary.Concat_StrStr` (`KismetSystemLibrary.GetDisplayName` (`self.GetOwner`)) "Weapon Is Not Valid"))
      (`KismetArrayLibrary.Array_Clear` (`self.SocketName`)))))

(event `UpdateSocketLocation`
  ;[0 0.9829 1] UpdateSocketLocation,Culculate previous Location
  (for _array_element (`self.SocketName`)
    (`BlueprintMapLibrary.Map_Add` (`self.PreSocketLocation`) _array_element (`SceneComponent.GetSocketLocation` (`self.Mesh`) _array_element))))

(event `EnableTrace`
  (bind _ignoreactors (`self.IgnoreActors`))
  ;[0 1 0.01884] Enable And Disable Trace
  (set `self.OpenTrace?` true)
  (`KismetArrayLibrary.Array_Clear` _ignoreactors)
  (`KismetArrayLibrary.Array_Add` _ignoreactors (`self.GetOwner`)))

(event `DisableTrace`
  ;[0 1 0.01884] Enable And Disable Trace
  (set `self.OpenTrace?` false)
  (`KismetArrayLibrary.Array_Clear` (`self.IgnoreActors`)))

(event `PerfromTrace`
  (bind _mesh (`self.Mesh`))
  ;[1 0.07651 0] Perform Trace
  (for _array_element (`SceneComponent.GetAllSocketNames` _mesh)
    (bind _outhits (`KismetSystemLibrary.LineTraceMultiForObjects` (`BlueprintMapLibrary.Map_Find` (`self.PreSocketLocation`) _array_element) (`SceneComponent.GetSocketLocation` _mesh _array_element) (`self.CanEffectActors`) false (`self.IgnoreActors`) (`self.DebugType`)))
    (for _array_element_2 _outhits
      (bind (_bblockinghit _binitialoverlap _time _distance _location _impactpoint _normal _impactnormal _physmat _hitactor) (`GameplayStatics.BreakHitResult` _array_element_2))
      (if (`KismetSystemLibrary.DoesImplementInterface` _hitactor "/Game/CombatSystem/BluePrints/UserInterface/BPI_CanbeAttackable.BPI_CanbeAttackable_C")
        (break)))
    (`KismetArrayLibrary.Array_Add` (`self.IgnoreActors`) _hitactor)
    (`self.OnHit` _array_element_2)))

(event `self.ReceiveTick`
  (params (DeltaSeconds :type "Float (single-precision)"))
  ;[0.496 0.412 0.09006] Event Tick
  (if (`self.OpenTrace?`)
    (`|ExecutionSequence`
      (:`then_0`
        (`self.PerfromTrace`))
      (:`then_1`
        (`self.UpdateSocketLocation`)))))