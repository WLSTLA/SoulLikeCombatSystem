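; BPC_MontagesManager is a combat component that looks up animation montages by weapon type and action.
; It reads rows from a weapon data table, named after the weapon enum, and stores the current weapon as the fallback for lookups.
; Queries return the montage at a given index, or the last valid index, for an action.
; BeginPlay prints a warning naming the owner if the table is unset.
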(event `self.ReceiveBeginPlay`
  (if (not (`KismetSystemLibrary.IsValid` (`self.WeaponDataTable`)))
    (`KismetSystemLibrary.PrintString` (`KismetStringLibrary.Concat_StrStr` "DaTable On" (`KismetSystemLibrary.GetDisplayName` (`self.GetOwner`)) "Is NULL!"))))

(fn `GetActionLastIndex`
  (params (MontageAction :type "/Game/CombatSystem/BluePrints/Enumerations/Character/E_MontageAction Enum" :default "NewEnumerator0") (WeaponType :type "/Game/CombatSystem/BluePrints/Enumerations/Character/E_WeaponType Enum" :default "NewEnumerator3"))
  (returns (`IsFind?` :type Boolean) (`Last Index` :type Integer))
  (locals (MontageAction_Local :type "/Game/CombatSystem/BluePrints/Enumerations/Character/E_MontageAction Enum" :default "NewEnumerator0") (LocalWeaponType :type "/Game/CombatSystem/BluePrints/Enumerations/Character/E_WeaponType Enum" :default "NewEnumerator3"))
  (set `local.MontageAction_Local` MontageAction)
  (bind _output_get (set `local.LocalWeaponType` WeaponType))
  (`/Engine/EditorBlueprintResources/StandardMacros.IsValid` (`self.WeaponDataTable`)
    (:`Is Valid`
      (bind _returnvalue (`|GetDataTableRow` (`self.WeaponDataTable`) (`self.GetWeaponName` (select `bool` (`|EnumInequality` _output_get "NewEnumerator3") :`false` (`self.CurrentWeapon`) :`true` (`local.LocalWeaponType`))))
        (:`then`
          (for _array_element (`.WeaponMontages_6_143BB11F46BE98376516C5B9796BC30F` (break `/Game/CombatSystem/BluePrints/Structures/S_WeaponInfo` _returnvalue))
            (bind (_montageaction _montages) (break `/Game/CombatSystem/BluePrints/Structures/S_WeaponMontage` _array_element))
            (if (== (`local.MontageAction_Local`) _montageaction)
              (return true (`KismetArrayLibrary.Array_LastIndex` _montages)))))
        (:`RowNotFound`
          _)))
    (:`Is Not Valid`
      _))
  (return false 0))

(fn `GetMontageForAction`
  (params (MontageAction :type "/Game/CombatSystem/BluePrints/Enumerations/Character/E_MontageAction Enum" :default "NewEnumerator0") (Index :type Integer) (WeaponType :type "/Game/CombatSystem/BluePrints/Enumerations/Character/E_WeaponType Enum" :default "NewEnumerator3"))
  (returns (Action :type "AnimMontage Object Reference") (`Success?` :type Boolean))
  (locals (MontageAction_Local :type "/Game/CombatSystem/BluePrints/Enumerations/Character/E_MontageAction Enum" :default "NewEnumerator0") (Index_Local :type Integer) (NewWeapon_Local :type "/Game/CombatSystem/BluePrints/Enumerations/Character/E_WeaponType Enum" :default "NewEnumerator3"))
  (set `local.MontageAction_Local` MontageAction)
  (set `local.Index_Local` Index)
  (bind _output_get (set `local.NewWeapon_Local` WeaponType))
  (`/Engine/EditorBlueprintResources/StandardMacros.IsValid` (`self.WeaponDataTable`)
    (:`Is Valid`
      (bind _returnvalue (`|GetDataTableRow` (`self.WeaponDataTable`) (`self.GetWeaponName` (select `bool` (`|EnumInequality` _output_get "NewEnumerator3") :`false` (`self.CurrentWeapon`) :`true` (`local.NewWeapon_Local`))))
        (:`then`
          (for _array_element (`.WeaponMontages_6_143BB11F46BE98376516C5B9796BC30F` (break `/Game/CombatSystem/BluePrints/Structures/S_WeaponInfo` _returnvalue))
            (bind (_montageaction _montages) (break `/Game/CombatSystem/BluePrints/Structures/S_WeaponMontage` _array_element))
            (if (`|EnumEquality` _montageaction (`local.MontageAction_Local`))
              (for (_array_element_2 _array_index) _montages
                (if (== _array_index (`local.Index_Local`))
                  (return _array_element_2 true)))
              (return null false))))
        (:`RowNotFound`
          _)))
    (:`Is Not Valid`
      _))
  (return null false))

(fn `GetWeaponName`
  (params (WeaponType :type "/Game/CombatSystem/BluePrints/Enumerations/Character/E_WeaponType Enum" :default "NewEnumerator3"))
  (returns (WeaponName :type Name))
  (return (`KismetStringLibrary.Conv_StringToName` (`|GetEnumeratorNameAsString` WeaponType))))

(fn `UpdateWeaponType`
  (params (`Weapon Type` :type "/Game/CombatSystem/BluePrints/Enumerations/Character/E_WeaponType Enum" :default "NewEnumerator3"))
  (returns (`IsFind?` :type Boolean))
  (locals (LocalWeaponType :type "/Game/CombatSystem/BluePrints/Enumerations/Character/E_WeaponType Enum"))
  (bind _output_get (set `local.LocalWeaponType` `Weapon Type`))
  (bind _returnvalue (`|GetDataTableRow` (`self.WeaponDataTable`) (`self.GetWeaponName` _output_get))
    (:`then`
      (set `self.CurrentWeapon` (`.WeaponType_2_0C78E0164BCCFC9EF37AFFA2E005AC38` (break `/Game/CombatSystem/BluePrints/Structures/S_WeaponInfo` _returnvalue)))
      (return true))
    (:`RowNotFound`
      (set `self.CurrentWeapon` "NewEnumerator3")
      (return false))))