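; Inventory component for the Player that stores weapons up to a size limit.
; On BeginPlay it caches the owning Player and applies the initial capacity, printing an error if the owner cast fails.
; AddWeapon appends only while space remains and returns whether it succeeded, with capacity adjustable through UpdateWeaponInventorySize.
; ContainWeapon reports whether any stored weapon's class exactly matches a given class.
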(event `self.ReceiveBeginPlay`
  (bind _asplayer (cast `/Game/CombatSystem/BluePrints/Player/Player` (`self.GetOwner`))
    (:`then`
      (set `self.OwnerRef` _asplayer)
      (`self.UpdateWeaponInventorySize` (`self.InitialWeaponINSize`)))
    (:`CastFailed`
      (`KismetSystemLibrary.PrintString` "Inventory获取Owner失败"))))

(fn `AddWeapon`
  (params (Weapon :type "/Game/CombatSystem/BluePrints/Core/Item/Weapon/BP_WeaponMaster Object Reference (by ref)"))
  (returns (`AddSuccess?` :type Boolean))
  (if (< (`KismetArrayLibrary.Array_Length` (`self.WeaponInventory`)) (`self.CurrentWeaponINSize`))
    (`KismetArrayLibrary.Array_Add` (`self.WeaponInventory`) Weapon)
    (return true)
    (else
      (return false))))

(fn `ContainWeapon?`
  (params (WeaponClass :type "/Game/CombatSystem/BluePrints/Core/Item/Weapon/BP_WeaponMaster Class Reference"))
  (returns (`Contain?` :type Boolean))
  (for _array_element (`self.WeaponInventory`)
    (if (== (`GameplayStatics.GetObjectClass` _array_element) WeaponClass)
      (return true)))
  (return false))

(fn `UpdateWeaponInventorySize`
  (params (InputSize :type Integer))
  (set `self.CurrentWeaponINSize` InputSize)
  (return))