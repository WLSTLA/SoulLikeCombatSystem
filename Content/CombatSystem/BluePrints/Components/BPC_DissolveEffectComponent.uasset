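; Actor component that dissolves a combat character's meshes after death, then tells the owner it can be destroyed.
; Meshes are registered only if the owner implements BPI_CanbeAttackable.
; BeginDissolved waits for the death animation, applies the dissolve material and starts a looping timer.
; Each tick eases the dissolve parameter via FInterpTo on per-slot dynamic materials until near full, then stops and notifies the owner.
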(event `GetOnwerNeedDissolveMesh`
  (params (NeedDissolveMesh :type "PrimitiveComponent Object Reference (by ref)"))
  (bind _dissolvemesh (`self.DissolveMesh`))
  ;[0.3359 1 0] Initial
  (if (`KismetSystemLibrary.DoesImplementInterface` (`self.GetOwner`) "/Game/CombatSystem/BluePrints/UserInterface/BPI_CanbeAttackable.BPI_CanbeAttackable_C")
    (`KismetArrayLibrary.Array_AddUnique` _dissolvemesh NeedDissolveMesh)
    (if (not (> (`KismetArrayLibrary.Array_Length` _dissolvemesh) 0))
      (`KismetSystemLibrary.PrintString` "DissolveArray Is Empty！"))
    (else
      (`KismetSystemLibrary.PrintString` "DissolveBPC Owner Doesnt Implement specific BPI"))))

(event `ChangeMaterialToDissolve`
  (bind _dissolvemesh (`self.DissolveMesh`))
  ;[0 1 0.5078] 切换成消散的材质
  (`/Engine/EditorBlueprintResources/StandardMacros.IsValid` (`self.DissolveEffect`)
    (:`Is Valid`
      (for _array_element _dissolvemesh
        (for _index (range (`PrimitiveComponent.GetNumMaterials` _array_element))
          (`PrimitiveComponent.SetMaterial` _dissolvemesh _index (`self.DissolveEffect`)))))))

(event `BeginDissolved`
  ;[0.4766 1 0] BeginDissolve
  ;;[0 0.9766 1] 等待角色播放完死亡动画后
  (`KismetSystemLibrary.Delay` 4.0)
  (`self.ChangeMaterialToDissolve`)
  (bind _returnvalue (`KismetSystemLibrary.K2_SetTimer` null "UpdateDissolveMaterialParam" (`self.DissolveTick`) true))
  (set `self.DissolveTimer` _returnvalue))

(fn `UpdateDissolveMaterialParam`
  (`/Engine/EditorBlueprintResources/StandardMacros.IsValid` (`self.DissolveEffect`)
    (:`Is Valid`
      (set `self.DissolveAmount` (`KismetMathLibrary.FInterpTo` (`self.DissolveAmount`) 1.0 (`GameplayStatics.GetWorldDeltaSeconds`) (`self.DissolveInterpSpeed`)))
      (for _array_element (`self.DissolveMesh`)
        (for _index (range (`PrimitiveComponent.GetNumMaterials` _array_element))
          (bind _returnvalue (`PrimitiveComponent.CreateDynamicMaterialInstance` _array_element _index (`self.DissolveEffect`) "None"))
          (`MaterialInstanceDynamic.SetScalarParameterValue` _returnvalue (`self.DissAmountName`) (`self.DissolveAmount`))))
      (if (`KismetMathLibrary.NearlyEqual_FloatFloat` (`self.DissolveAmount`) 1.0 0.1)
        (`KismetSystemLibrary.K2_ClearAndInvalidateTimerHandle` (`self.DissolveTimer`))
        (set `self.DissolveAmount` 0.0)
        (message `/Game/CombatSystem/BluePrints/UserInterface/BPI_CanbeAttackable.CanBeDestroyEvent` (`self.GetOwner`))
        (return)))
    (:`Is Not Valid`
      (`KismetSystemLibrary.PrintString` "DissolveEffect is Empty!")
      (`KismetSystemLibrary.K2_ClearAndInvalidateTimerHandle` (`self.DissolveTimer`)))))