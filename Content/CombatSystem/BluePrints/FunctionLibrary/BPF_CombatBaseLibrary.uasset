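; Blueprint function library of helpers for the combat system.
; CalculateHitDirection classifies where an attacker stands relative to the receiver, using dot products on its forward vector for front or back and its right vector for either side, defaulting to front for invalid actors.
; ChangeAttackTypeToAction maps attack types to action enum values, with Null, Execution and Ambush sharing the light-attack result.
; GetDistanceTo wraps the actor distance query with validity checks.
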(fn `CalculateHitDirection`
  (params (Attacker :type "Actor Object Reference") (Reciver :type "Actor Object Reference"))
  (returns (Direction :type "/Game/CombatSystem/BluePrints/Enumerations/Character/E_HitDirection Enum"))
  (locals (LocalAttacker :type "Actor Object Reference") (LocalReciver :type "Actor Object Reference") (HitDirection :type "/Game/CombatSystem/BluePrints/Enumerations/Character/E_HitDirection Enum"))
  (bind _localreciver (`local.LocalReciver`))
  (bind _returnvalue (`KismetMathLibrary.Dot_VectorVector` (`KismetMathLibrary.Normal` (- (`Actor.K2_GetActorLocation` (`local.LocalAttacker`)) (`Actor.K2_GetActorLocation` _localreciver))) (`Actor.GetActorForwardVector` _localreciver)))
  (if (and (`KismetSystemLibrary.IsValid` Attacker) (`KismetSystemLibrary.IsValid` Reciver))
    (set `local.LocalAttacker` Attacker)
    (set `local.LocalReciver` Reciver)
    (set `local.HitDirection` "NewEnumerator3")
    (if (>= _returnvalue 0.5)
      (set `local.HitDirection` "NewEnumerator3")
      (elif (<= _returnvalue -0.5)
        (set `local.HitDirection` "NewEnumerator4")
        (elif (>= (`KismetMathLibrary.Dot_VectorVector` (`KismetMathLibrary.Normal` (- (`Actor.K2_GetActorLocation` (`local.LocalAttacker`)) (`Actor.K2_GetActorLocation` (`local.LocalReciver`)))) (`Actor.GetActorRightVector` (`local.LocalReciver`))) 0.0)
          (set `local.HitDirection` "NewEnumerator8")
          (else
            (set `local.HitDirection` "NewEnumerator7")))))
    (else
      (set `local.HitDirection` "NewEnumerator3")))
  (return (`local.HitDirection`)))

(fn `ChangeAttackTypeToAction`
  (params (AttackType :type "/Game/CombatSystem/BluePrints/Enumerations/Character/E_AttackType Enum" :default "NewEnumerator4"))
  (returns (ActionType :type "/Game/CombatSystem/BluePrints/Enumerations/Character/E_MontageAction Enum"))
  (return (select `/Game/CombatSystem/BluePrints/Enumerations/Character/E_AttackType` AttackType :`NewEnumerator4` "NewEnumerator0" :`NewEnumerator0` "NewEnumerator0" :`NewEnumerator1` "NewEnumerator1" :`NewEnumerator2` "NewEnumerator2" :`NewEnumerator3` "NewEnumerator3" :`NewEnumerator5` "NewEnumerator0" :`NewEnumerator6` "NewEnumerator0" :!type "/Game/CombatSystem/BluePrints/Enumerations/Character/E_MontageAction Enum")))

(fn `GetDistanceTo`
  (params (From :type "Actor Object Reference") (To :type "Actor Object Reference"))
  (returns (Distance :type "Float (double-precision)"))
  (locals (LocalFrom :type "Actor Object Reference") (LocalTo :type "Actor Object Reference"))
  (if (and (`KismetSystemLibrary.IsValid` From) (`KismetSystemLibrary.IsValid` To))
    (bind _output_get (set `local.LocalFrom` From))
    (bind _output_get_2 (set `local.LocalTo` To))
    (return (`Actor.GetDistanceTo` _output_get _output_get_2))))