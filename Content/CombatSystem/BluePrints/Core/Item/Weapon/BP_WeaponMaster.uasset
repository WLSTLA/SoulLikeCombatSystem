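; BP_WeaponMaster is a data-driven weapon item, apparently the base for the combat system's weapons.
; Its construction script looks up the DT_WeaponInfo row named after its WeaponType enum, so the type selects the weapon's setup.
; A found row fills WeaponInfo with montages, damage, play rate, sockets and mesh, then applies that mesh to ItemMesh.
; The event graph holds only disabled placeholder events.
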(fn `UserConstructionScript`
  (bind (_weaponinfo_weaponname _weaponinfo_weapontype) (break `/Game/CombatSystem/BluePrints/Structures/S_WeaponInfo` (`self.WeaponInfo`)))
  (`parent.UserConstructionScript`)
  (bind _returnvalue (`|GetDataTableRow` "/Game/CombatSystem/BluePrints/DataTables/DT_WeaponInfo.DT_WeaponInfo" (`KismetStringLibrary.Conv_StringToName` (`|GetEnumeratorNameAsString` _weaponinfo_weapontype)))
    (:`then`
      (bind (_weaponname _weapontype _weaponmontages _basedamage _playrate _equipsocket _unequipsocket _weaponmesh) (break `/Game/CombatSystem/BluePrints/Structures/S_WeaponInfo` _returnvalue))
      (set `self.WeaponInfo` (make `/Game/CombatSystem/BluePrints/Structures/S_WeaponInfo` _weaponname _weapontype _weaponmontages _basedamage _playrate _equipsocket _unequipsocket _weaponmesh))
      (`StaticMeshComponent.SetStaticMesh` (`self.ItemMesh`) _weaponmesh))))