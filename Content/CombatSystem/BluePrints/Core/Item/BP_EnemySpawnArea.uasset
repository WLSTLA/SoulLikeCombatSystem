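; BP_EnemySpawnArea is a placeable area that spawns a batch of combat enemies around itself.
; SpawnEnemy spawns SpawnNumber Enemy_Base actors with the configured WeaponClass at random reachable nav points within Range.
; Each enemy starts its behavior tree and immediately receives player 0 as its perception target.
; The construction script sizes the SpawnArea box from Range, although spawning uses it as a radius.
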(event `SpawnEnemy`
  (for _ (range (+ (`KismetMathLibrary.FTrunc` (- (`self.SpawnNumber`) 1.0)) 1))
    (bind _returnvalue (`|SpawnActorFromClass` "/Game/CombatSystem/BluePrints/Enemy/Enemy_Base.Enemy_Base_C" (`KismetMathLibrary.MakeTransform` (`NavigationSystemV1.K2_GetRandomReachablePointInRadius` (`self.K2_GetActorLocation`) (`self.Range`) null null)) "Undefined" "OverrideRootScale" null (`self.Weapon Class`) null))
    (`AIController.RunBehaviorTree` (`/Game/CombatSystem/BluePrints/Enemy/Enemy_Base.AIController` _returnvalue) (`/Game/CombatSystem/BluePrints/Enemy/Enemy_Base.BehaviorTree` _returnvalue))
    (`/Game/CombatSystem/BluePrints/Enemy/Enemy_Base.SetTargetOnPerception` _returnvalue (`GameplayStatics.GetPlayerCharacter` 0))))

(fn `UserConstructionScript`
  (bind _range (`self.Range`))
  (`BoxComponent.SetBoxExtent` (`self.SpawnArea`) (`KismetMathLibrary.MakeVector` _range _range 10.0) true))