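; Game base Blueprint, apparently the game mode, that respawns the player whenever the Player character is destroyed.
; On BeginPlay it gathers PlayerStart actors and binds RespawnEvent to the character's OnDestroyed.
; RespawnEvent spawns a new Player at the first PlayerStart's location with zero rotation and possesses it with player controller 0.
; It then rebinds through BindSpawn for the next death and calls CallPlayerSpawn to signal the spawn.
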(event `self.ReceiveBeginPlay`
  (bind _outactors (`GameplayStatics.GetAllActorsOfClass` "/Script/Engine.PlayerStart" :!label _label))
  (bind _asplayer (cast `/Game/CombatSystem/BluePrints/Player/Player` (`GameplayStatics.GetPlayerCharacter` 0)))
  (add `self.OnDestroyed` _asplayer (delegate `RespawnEvent`)))

(event `BindSpawn`
  (goto _label))

(event `RespawnEvent` :!signature `self.OnDestroyed`
  (params (DestroyedActor :type "Actor Object Reference"))
  (bind _returnvalue (`|SpawnActorFromClass` "/Game/CombatSystem/BluePrints/Player/Player.Player_C" (`KismetMathLibrary.MakeTransform` (`self.K2_GetActorLocation` (`|GetArrayItem` (stale `self.ReceiveBeginPlay` _outactors)))) "Undefined" "OverrideRootScale" null null))
  (`Controller.Possess` (`GameplayStatics.GetPlayerController` 0) _returnvalue)
  (`self.BindSpawn`)
  (`self.PlayerSpawn`))

(fn `UserConstructionScript`)